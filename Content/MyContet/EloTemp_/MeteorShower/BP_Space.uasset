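; BP_Space spawns meteor shower effects at random places inside a box area.
; On BeginPlay it starts a looping timer whose interval is picked once between the min and max spawn delay, so the period stays fixed afterwards.
; Each tick of that timer spawns the NS_MeteorShower system at a random point in the MeteorShowerSpawnArea box with a random rotation.
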(event Custom|Spawn
  (bind _meteorshower_spawnarea (Variables|Default|GetMeteorShower_SpawnArea))
  ;[1 1 1] Random Spawn MeteorShower
  (Niagara|SpawnSystematLocation "/Game/MyContet/EloTemp_/MeteorShower/NS_MeteorShower.NS_MeteorShower" (Math|Random|RandomPointinBoundingBox (Transformation|GetWorldLocation _meteorshower_spawnarea) (Variables|/Script/Engine.BoxComponent|GetBoxExtent _meteorshower_spawnarea)) (Math|Random|RandomRotator true)))

(event EventBeginPlay
  ;[1 1 1] Random Spawn MeteorShower
  (Utilities|Time|SetTimerbyEvent (delegate Custom|Spawn) (Math|Random|RandomFloatinRange (Variables|MeteorShower|GetMinSpawnDelay) (Variables|MeteorShower|GetMaxSpawnDelay)) true true))

(fn ConstructionScript)