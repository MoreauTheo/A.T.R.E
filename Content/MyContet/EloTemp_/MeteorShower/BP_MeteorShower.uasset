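; BP_MeteorShower is an actor that spawns meteor shower Niagara effects at random spots inside its box area.
; On BeginPlay it starts a looping timer with a delay picked once at random between a minimum and maximum.
; Each tick of that timer spawns NS_MeteorShower at a random point within the SpawnArea box, with a random rotation.
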(event Custom|Spawn
  (bind _spawnarea (Variables|Default|GetSpawnArea))
  ;[1 1 1] Random Spawn MeteorShower
  (Niagara|SpawnSystematLocation "/Game/MyContet/EloTemp_/MeteorShower/NS_MeteorShower.NS_MeteorShower" (Math|Random|RandomPointinBoundingBox (Transformation|GetWorldLocation _spawnarea) (Variables|/Script/Engine.BoxComponent|GetBoxExtent _spawnarea)) (Math|Random|RandomRotator true)))

(event EventBeginPlay
  ;[1 1 1] Random Spawn MeteorShower
  (Utilities|Time|SetTimerbyEvent (delegate Custom|Spawn) (Math|Random|RandomFloatinRange (Variables|Default|GetMinSpawnDelay) (Variables|Default|GetMaxSpawnDelay)) true true))

(fn ConstructionScript)