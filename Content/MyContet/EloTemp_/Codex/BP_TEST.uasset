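; Test actor that previews animations for a screen of body icons (Pyraxis, Hexor, Theron, Zentor) through debug keys.
; Tick spins the icons, while keys resize Pyraxis, toggle a highlight mesh, and slide a support mesh while rescaling the screen.
; BeginPlay enables input and resets the validation flipbooks to stopped.
; Theron and Zentor unlock keys play a flipbook once, spawn a Niagara burst and scale an icon via timeline.
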(event EventTick
  (params (DeltaSeconds :type Float%20%28single-precision%29))
  (bind _speed (Variables|Default|GetSpeed))
  (bind _returnvalue (* _speed DeltaSeconds))
  (bind _returnvalue_2 (Math|Rotator|MakeRotator _returnvalue 0.0 0.0))
  ;[1 1 1] Bodie Icon Rotation
  (Transformation|AddLocalRotation (Variables|Default|GetSM_PyraxisIcon) _returnvalue_2 false false)
  (Transformation|AddLocalRotation (Variables|Default|GetSM_HexorIcon) _returnvalue_2 false false)
  (Transformation|AddLocalRotation (Variables|Default|GetSM_TheronIcon5) _returnvalue_2 false false)
  (Transformation|AddLocalRotation (Variables|Default|GetSM_ZentorIcon) _returnvalue_2 false false))

(event EventBeginPlay
  (Input|EnableInput (Game|GetPlayerController 0))
  ;[1 0.502 0] Unlock
  (CallFunction|StopFlipbook))

(event Input|KeyboardEvents|F
  (params (Key :type Key%20Structure :default "None"))
  (bind _sm_pyraxis (Variables|Default|GetSM_Pyraxis))
  ;[0.644 1 0] TEMP - Animation over
  (:Pressed
    (Transformation|SetWorldScale3D _sm_pyraxis (+ (Transformation|GetWorldScale _sm_pyraxis) "0.012000,0.012000,0.000000"))))

(event Input|KeyboardEvents|D
  (params (Key :type Key%20Structure :default "None"))
  (bind _sm_rightsuport (Variables|Default|GetSM_RightSuport))
  (:Pressed
    ;[1 1 1] Right Translation Suport
    (bind _newtrack_0 (Timeline|RightTranslation PlayFromStart)
      (:Update
        (Transformation|SetWorldLocation _sm_rightsuport (.location (Math|Transform|Lerp(Transform) (Math|Transform|MakeTransform (Transformation|GetWorldLocation _sm_rightsuport) "0, 0, 0" "1.000000,1.000000,1.000000") (Math|Transform|MakeTransform (Transformation|GetWorldLocation (Variables|Default|GetSM_LeftSuport)) "0, 0, 0" "1.000000,1.000000,1.000000") _newtrack_0)) false false)
        (Transformation|SetWorldScale3D (Variables|Default|GetSM_Screen) "1.000000,1.000000,1.000000")))))

(event Input|KeyboardEvents|L
  (params (Key :type Key%20Structure :default "None"))
  ;[1 0.4416 0] Unlock
  (:Pressed
    (CallFunction|UnlockTheron)
    (bind _newtrack_2 (Timeline|ScaleIcon Play)
      (:Update
        (Transformation|SetWorldScale3D (Variables|Default|GetSM_ZentorIcon2) _newtrack_2)))))

(event Input|KeyboardEvents|E
  (params (Key :type Key%20Structure :default "None"))
  (bind _sm_rightsuport (Variables|Default|GetSM_RightSuport))
  (:Pressed
    ;[1 1 1] Left Translation Suport
    (bind _newtrack_0 (Timeline|LeftTranslation PlayFromStart)
      (:Update
        (Transformation|SetWorldLocation _sm_rightsuport (.location (Math|Transform|Lerp(Transform) (Math|Transform|MakeTransform (Transformation|GetWorldLocation _sm_rightsuport) "0, 0, 0" "1.000000,1.000000,1.000000") (Math|Transform|MakeTransform (+ (Transformation|GetWorldLocation (Variables|Default|GetSM_LeftSuport)) "250.000000,0.000000,0.000000") "0, 0, 0" "1.000000,1.000000,1.000000") _newtrack_0)) false false)
        (Transformation|SetWorldScale3D (Variables|Default|GetSM_Screen) (Variables|ScreenAnimation|GetScreenTranslationAmount))))))

(event Input|KeyboardEvents|G
  (params (Key :type Key%20Structure :default "None"))
  (bind _sm_pyraxis (Variables|Default|GetSM_Pyraxis))
  ;[0.644 1 0] TEMP - Animation over
  (:Pressed
    (Transformation|SetWorldScale3D _sm_pyraxis (- (Transformation|GetWorldScale _sm_pyraxis) "0.012000,0.012000,0.000000"))))

(event Input|KeyboardEvents|A
  (params (Key :type Key%20Structure :default "None"))
  ;[1 0.6933 0] Active Highlight
  (:Pressed
    (Development|SetHiddeninGame (Variables|Default|GetSM_Feet1) false false)))

(event Input|KeyboardEvents|B
  (params (Key :type Key%20Structure :default "None"))
  ;[1 0.6933 0] Active Highlight
  (:Pressed
    (Development|SetHiddeninGame (Variables|Default|GetSM_Feet1) true false)))

(event Input|KeyboardEvents|C
  (params (Key :type Key%20Structure :default "None"))
  ;[1 0.4416 0] Unlock
  (:Pressed
    (CallFunction|UnlockZentor)
    (bind _newtrack_2 (Timeline|Timeline Play)
      (:Update
        (Transformation|SetWorldScale3D (Variables|Default|GetSM_ZentorIcon1) _newtrack_2)))))

(fn ConstructionScript)

(fn StopFlipbook
  (bind _validationsprite2 (Variables|Default|GetValidationSprite2))
  (bind _validationsprite3 (Variables|Default|GetValidationSprite3))
  (bind _validationsprite4 (Variables|Default|GetValidationSprite4))
  (bind _validationsprite5 (Variables|Default|GetValidationSprite5))
  (bind _validationsprite6 (Variables|Default|GetValidationSprite6))
  (bind _validationsprite7 (Variables|Default|GetValidationSprite7))
  (bind _validationsprite (Variables|Default|GetValidationSprite))
  (bind _validationsprite1 (Variables|Default|GetValidationSprite1))
  (Utilities|FlowControl|DoOnce false
    (:Completed
      (Utilities|FlowControl|Sequence
        (:then_0
          (Components|Timeline|PlayfromStart _validationsprite)
          (if (== (Class|PaperFlipbookComponent|GetPlaybackPositioninFrames _validationsprite) 0)
            _
            (else
              _))
          (Audio|Components|Audio|Stop _validationsprite))
        (:then_1
          (Components|Timeline|PlayfromStart _validationsprite1)
          (if (== (Class|PaperFlipbookComponent|GetPlaybackPositioninFrames _validationsprite1) 0)
            _
            (else
              _))
          (Audio|Components|Audio|Stop _validationsprite1))
        (:then_2
          (Components|Timeline|PlayfromStart _validationsprite2)
          (if (== (Class|PaperFlipbookComponent|GetPlaybackPositioninFrames _validationsprite2) 0)
            _
            (else
              _))
          (Audio|Components|Audio|Stop _validationsprite2))
        (:then_3
          (Components|Timeline|PlayfromStart _validationsprite3)
          (if (== (Class|PaperFlipbookComponent|GetPlaybackPositioninFrames _validationsprite3) 0)
            _
            (else
              _))
          (Audio|Components|Audio|Stop _validationsprite3))
        (:then_4
          (Components|Timeline|PlayfromStart _validationsprite4)
          (if (== (Class|PaperFlipbookComponent|GetPlaybackPositioninFrames _validationsprite4) 0)
            _
            (else
              _))
          (Audio|Components|Audio|Stop _validationsprite4))
        (:then_5
          (Components|Timeline|PlayfromStart _validationsprite5)
          (if (== (Class|PaperFlipbookComponent|GetPlaybackPositioninFrames _validationsprite5) 0)
            _
            (else
              _))
          (Audio|Components|Audio|Stop _validationsprite5))
        (:then_6
          (Components|Timeline|PlayfromStart _validationsprite6)
          (if (== (Class|PaperFlipbookComponent|GetPlaybackPositioninFrames _validationsprite6) 0)
            _
            (else
              _))
          (Audio|Components|Audio|Stop _validationsprite6))
        (:then_7
          (Components|Timeline|PlayfromStart _validationsprite7)
          (if (== (Class|PaperFlipbookComponent|GetPlaybackPositioninFrames _validationsprite7) 0)
            _
            (else
              _))
          (Audio|Components|Audio|Stop _validationsprite7))))))

(fn UnlockTheron
  (bind _validationsprite (Variables|Default|GetValidationSprite))
  (Components|Timeline|PlayfromStart _validationsprite)
  (Components|Timeline|SetLooping _validationsprite false)
  (Niagara|SpawnSystematLocation "/Game/MyContet/EloTemp_/Unlock/NS_Unlock.NS_Unlock" (Transformation|GetWorldLocation _validationsprite) "0.000000,0.000000,90.000000"))

(fn UnlockZentor
  (bind _validationsprite6 (Variables|Default|GetValidationSprite6))
  (Components|Timeline|PlayfromStart _validationsprite6)
  (Components|Timeline|SetLooping _validationsprite6 false)
  (Niagara|SpawnSystematLocation "/Game/MyContet/EloTemp_/Unlock/NS_Unlock.NS_Unlock" (Transformation|GetWorldLocation _validationsprite6) "0.000000,0.000000,90.000000"))