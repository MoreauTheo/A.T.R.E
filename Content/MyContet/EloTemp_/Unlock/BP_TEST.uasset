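; Test actor that previews animations for what appears to be an unlock or selection screen, triggered by debug keys A to G.
; Keys toggle a feet highlight, play a validation sprite with enlarged text, and nudge the Pyraxis mesh scale.
; Two timelines lerp the right support from its current location toward the left support, with or without an offset, while setting the screen scale.
; Tick continuously rotates four body icons.
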(event EventTick
  (params (DeltaSeconds :type Float%20%28single-precision%29))
  (bind _speed (Variables|Default|GetSpeed))
  (bind _returnvalue (* _speed DeltaSeconds))
  (bind _returnvalue_2 (Math|Rotator|MakeRotator _returnvalue 0.0 0.0))
  ;[1 1 1] Bodie Icon Rotation
  (Transformation|AddLocalRotation (Variables|Default|GetSM_PyraxisIcon) _returnvalue_2 false false)
  (Transformation|AddLocalRotation (Variables|Default|GetSM_HexorIcon) _returnvalue_2 false false)
  (Transformation|AddLocalRotation (Variables|Default|GetSM_TheronIcon5) _returnvalue_2 false false)
  (Transformation|AddLocalRotation (Variables|Default|GetSM_ZentorIcon) _returnvalue_2 false false))

(event EventBeginPlay
  (Input|EnableInput (Game|GetPlayerController 0)))

(event Input|KeyboardEvents|F
  (params (Key :type Key%20Structure))
  (bind _sm_pyraxis (Variables|Default|GetSM_Pyraxis))
  ;[1 1 1] Over button
  ;;[0 0 0] TEMP - Animation over
  (:Pressed
    (Transformation|SetWorldScale3D _sm_pyraxis (+ (Transformation|GetWorldScale _sm_pyraxis) "0.012000,0.012000,0.000000"))))

(event Input|KeyboardEvents|D
  (params (Key :type Key%20Structure))
  (bind _sm_rightsuport (Variables|Default|GetSM_RightSuport))
  (:Pressed
    ;[1 1 1] Right Translation Suport
    (bind _newtrack_0 (Timeline|RightTranslation PlayFromStart)
      (:Update
        (Transformation|SetWorldLocation _sm_rightsuport (.location (Math|Transform|Lerp(Transform) (Math|Transform|MakeTransform (Transformation|GetWorldLocation _sm_rightsuport) "0, 0, 0" "1.000000,1.000000,1.000000") (Math|Transform|MakeTransform (Transformation|GetWorldLocation (Variables|Default|GetSM_LeftSuport)) "0, 0, 0" "1.000000,1.000000,1.000000") _newtrack_0)) false false)
        (Transformation|SetWorldScale3D (Variables|Default|GetSM_Screen) "1.000000,1.000000,1.000000")))))

(event Input|KeyboardEvents|E
  (params (Key :type Key%20Structure))
  (bind _sm_rightsuport (Variables|Default|GetSM_RightSuport))
  (:Pressed
    ;[1 1 1] Left Translation Suport
    (bind _newtrack_0 (Timeline|LeftTranslation PlayFromStart)
      (:Update
        (Transformation|SetWorldLocation _sm_rightsuport (.location (Math|Transform|Lerp(Transform) (Math|Transform|MakeTransform (Transformation|GetWorldLocation _sm_rightsuport) "0, 0, 0" "1.000000,1.000000,1.000000") (Math|Transform|MakeTransform (+ (Transformation|GetWorldLocation (Variables|Default|GetSM_LeftSuport)) "250.000000,0.000000,0.000000") "0, 0, 0" "1.000000,1.000000,1.000000") _newtrack_0)) false false)
        (Transformation|SetWorldScale3D (Variables|Default|GetSM_Screen) (Variables|ScreenAnimation|GetScreenTranslationAmount))))))

(event Input|KeyboardEvents|G
  (params (Key :type Key%20Structure))
  (bind _sm_pyraxis (Variables|Default|GetSM_Pyraxis))
  ;[1 1 1] Over button
  ;;[0 0 0] TEMP - Animation over
  (:Pressed
    (Transformation|SetWorldScale3D _sm_pyraxis (- (Transformation|GetWorldScale _sm_pyraxis) "0.012000,0.012000,0.000000"))))

(event Input|KeyboardEvents|A
  (params (Key :type Key%20Structure))
  ;[1 0.4387 0] Active Highlight
  (:Pressed
    (Development|SetHiddeninGame (Variables|Default|GetSM_Feet1) false false)))

(event Input|KeyboardEvents|B
  (params (Key :type Key%20Structure))
  ;[1 0.4387 0] Active Highlight
  (:Pressed
    (Development|SetHiddeninGame (Variables|Default|GetSM_Feet1) true false)))

(event Input|KeyboardEvents|C
  (params (Key :type Key%20Structure))
  (bind _validationsprite (Variables|Default|GetValidationSprite))
  ;[1 1 1] Over button
  ;;[1 0.359 0] Validation Animation Buton
  (:Pressed
    (Utilities|FlowControl|Sequence
      (:then_0
        (Development|SetHiddeninGame _validationsprite false false)
        (Components|Timeline|PlayfromStart _validationsprite)
        (Components|Timeline|SetLooping _validationsprite false))
      (:then_1
        (Rendering|Components|TextRender|SetWorldSize (Variables|Default|GetTextRender3) 5e+01)))))

(event Input|KeyboardEvents|H
  (params (Key :type Key%20Structure))
  ;[1 0.2955 0] Unlock Animation
)

(fn ConstructionScript)