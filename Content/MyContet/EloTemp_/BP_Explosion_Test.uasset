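; Test actor for a planet explosion, triggered by pressing C after enabling input from player controller 0 at BeginPlay.
; A timeline moves the planet mesh toward the Geometry Collection's location, interpolating from the mesh's current position on each update.
; The same key press immediately crumbles the collection's active clusters and, once only, activates a Niagara explosion effect after a short delay.
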(event EventBeginPlay
  ;[1 1 1] Key Test
  (Input|EnableInput (Game|GetPlayerController 0)))

(event Input|KeyboardEvents|C
  (params (Key :type Key%20Structure :default "None"))
  (bind _gc_test (Variables|Default|GetGC_Test))
  (bind _sm_planettest (Variables|Default|GetSM_PlanetTest))
  (:Pressed
    (Utilities|FlowControl|Sequence
      (:then_0
        ;[1 1 1] Planets Movment (Temp)
        (bind _newtrack_0 (Timeline|PlanetMovement Play)
          (:Update
            (Transformation|SetWorldLocation _sm_planettest (.location (Math|Transform|Lerp(Transform) (Math|Transform|MakeTransform (Transformation|GetWorldLocation _sm_planettest) "0, 0, 0" "1.000000,1.000000,1.000000") (Math|Transform|MakeTransform (Transformation|GetWorldLocation _gc_test) "0, 0, 0" "1.000000,1.000000,1.000000") _newtrack_0)) false false))))
      (:then_1
        ;[1 1 1] Planet Explosion
        (Class|GeometryCollectionComponent|CrumbleActiveClusters _gc_test)
        (Utilities|FlowControl|DoOnce false
          (:Completed
            (Utilities|FlowControl|Delay 1.1)
            (Components|Activation|Activate (Variables|Default|GetNS_Explosion_Test) false)))))))

(fn ConstructionScript)