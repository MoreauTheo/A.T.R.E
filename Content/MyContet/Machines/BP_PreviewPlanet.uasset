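; BP_PreviewPlanet is a preview planet actor that spins its mesh and registers itself with the crafting game mode.
; On BeginPlay, Init casts the game mode to GM_Craft and stores the actor in its PreviewPlanetTransform reference.
; A timeline then drives the planet mesh's relative yaw to animate the rotation.
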(event Custom|Movement_Body
  ;[1 1 1] Movement
  (bind _rotation_body (Timeline|T_Rotation_Body Play)
    (:Update
      (Transformation|SetRelativeRotation (Variables|Default|GetPlanetMesh) (Math|Rotator|MakeRotator 0.0 0.0 _rotation_body) false false))))

(event EventBeginPlay
  (CallFunction|Init)
  (CallFunction|MovementBody))

(event EventTick
  (params (DeltaSeconds :type Float%20%28single-precision%29))
  ;[1 1 1] Event tick
)

(fn ConstructionScript)

(fn Init
  (bind _asgm_craft (Utilities|Casting|CastToGM_Craft (Game|GetGameMode)))
  (Utilities|IsValid _asgm_craft
    (:Is%20Valid
      (bind _output_get (Variables|Default|SetGame%20Mode _asgm_craft))
      (Variables|/Game/MyContet/Blueprints/GM_Craft.GM_Craft_C|SetPreviewPlanetTransform _output_get self))
    (:Is%20Not%20Valid
      (Development|PrintString "GameMode non valide (BP_Lever)"))))