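; BP_ArrowScene is a clickable scene-change arrow that sends the GM_Craft camera to space and plays the scene-change sound.
; BeginPlay caches the sound manager and game mode, then puts a dynamic material on both arrow meshes.
; A click briefly dims their emissive and is locked against repeats for four seconds.
; The first click also advances the tutorial UI after a delay and clears the material's WeightMask.
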(event EventBeginPlay
  (bind _returnvalue (Actor|GetActorOfClass "/Game/MyContet/Sound/Bp_Sound_Manager.Bp_Sound_Manager_C"))
  (Variables|Default|SetSound_Mana_Ref _returnvalue)
  (bind _asgm_craft (Utilities|Casting|CastToGM_Craft (Game|GetGameMode)))
  (Variables|Default|SetGameMode _asgm_craft)
  (bind _returnvalue_2 (Rendering|Material|CreateDynamicMaterialInstance "/Game/MyContet/AssetLightsThéo/M_LightTest_Inst.M_LightTest_Inst" "None" "None" :!class /Script/Engine.KismetMaterialLibrary))
  (bind _output_get (Variables|Default|SetMatTuto _returnvalue_2))
  (Rendering|Material|SetScalarParameterValue _output_get "WeightMask" 0.0 :!class /Script/Engine.MaterialInstanceDynamic)
  (Rendering|Material|SetMaterial (Variables|Default|GetLightBeveled) 0 (Variables|Default|GetMatTuto))
  (Rendering|Material|SetMaterial (Variables|Default|GetFleche) 0 (Variables|Default|GetMatTuto)))

(event MouseInput|EventActorOnClicked
  (params (ButtonPressed :type Key%20Structure :default "None"))
  (bind _fleche (Variables|Default|GetFleche))
  (bind _gamemode (Variables|Default|GetGameMode))
  (bind _lightbeveled (Variables|Default|GetLightBeveled))
  (bind _ui (Variables|/Game/MyContet/Blueprints/GM_Craft.GM_Craft_C|GetUI _gamemode))
  (Utilities|FlowControl|DoOnce false :!label _label
    (:Completed
      (Default|ChangeScene (Variables|Default|GetSound_Mana_Ref))
      (Default|GotoSpace (Variables|/Game/MyContet/Blueprints/GM_Craft.GM_Craft_C|GetCam (Variables|Default|GetGameMode)))
      (Utilities|FlowControl|Sequence
        (:then_0
          (Utilities|FlowControl|Delay 2.5)
          (Utilities|FlowControl|DoOnce (Variables|Default|GetFirst)
            (:Completed
              (Rendering|Material|SetScalarParameterValue (Variables|Default|GetMatTuto) "WeightMask" 0.0 :!class /Script/Engine.MaterialInstanceDynamic)
              (Default|NextTuto _ui)
              (Default|SetnextDescription _ui))))
        (:then_1
          (Utilities|FlowControl|Delay 4.0)
          (goto _label Reset))
        (:then_2
          ;[1 1 1] On clicked Feedback
          (Rendering|Material|SetScalarParameterValueonMaterials _lightbeveled "EmissiveIntensity" 0.01)
          (Utilities|FlowControl|Delay 0.3)
          (Rendering|Material|SetScalarParameterValueonMaterials _lightbeveled "EmissiveIntensity" 1.0))
        (:then_3
          (Rendering|Material|SetScalarParameterValueonMaterials _fleche "EmissiveIntensity" 0.01)
          (Utilities|FlowControl|Delay 0.3)
          (Rendering|Material|SetScalarParameterValueonMaterials _fleche "EmissiveIntensity" 1.0))))))

(fn ConstructionScript)