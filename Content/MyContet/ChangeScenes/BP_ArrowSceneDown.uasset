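; Clickable scene-change arrow that moves the camera to the craft view, plays a sound and takes part in the tutorial.
; It registers itself with GM_Craft and gives its arrow and light meshes a shared dynamic highlight material.
; Clicks are locked briefly to prevent repeats.
; A DoOnce re-armed by AllowTutoDown lets a click advance the tutorial after a delay, moving the highlight to the Codex.
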(event Custom|AllowTutoDown
  (bind _gamemode (Variables|Default|GetGameMode))
  (bind _ui (Variables|/Game/MyContet/Blueprints/GM_Craft.GM_Craft_C|GetUI _gamemode))
  (bind _codex (Variables|/Game/MyContet/Blueprints/GM_Craft.GM_Craft_C|GetCodex _gamemode))
  (Utilities|FlowControl|DoOnce false) ; enters at Reset
)

(event EventBeginPlay
  (bind _asgm_craft (Utilities|Casting|CastToGM_Craft (Game|GetGameMode)))
  (Variables|Default|SetGameMode _asgm_craft)
  (bind _returnvalue (Actor|GetActorOfClass "/Game/MyContet/Sound/Bp_Sound_Manager.Bp_Sound_Manager_C"))
  (Variables|Default|SetSound_Mana_Ref _returnvalue)
  (bind _returnvalue_2 (Rendering|Material|CreateDynamicMaterialInstance "/Game/MyContet/ChangeScenes/M_LightTest.M_LightTest" "None" "None" :!class /Script/Engine.KismetMaterialLibrary))
  (bind _output_get (Variables|Default|SetMatTuto _returnvalue_2))
  (Rendering|Material|SetScalarParameterValue _output_get "WeightMask" 0.0 :!class /Script/Engine.MaterialInstanceDynamic)
  (Rendering|Material|SetMaterial (Variables|Default|GetLightBeveled) 0 (Variables|Default|GetMatTuto))
  (Rendering|Material|SetMaterial (Variables|Default|GetFleche) 0 (Variables|Default|GetMatTuto))
  (Variables|/Game/MyContet/Blueprints/GM_Craft.GM_Craft_C|SetArrowSceneDown (Variables|Default|GetGameMode) self))

(event MouseInput|EventActorOnClicked
  (params (ButtonPressed :type Key%20Structure :default "None"))
  (bind _gamemode (Variables|Default|GetGameMode))
  (bind _ui (Variables|/Game/MyContet/Blueprints/GM_Craft.GM_Craft_C|GetUI _gamemode))
  (bind _codex (Variables|/Game/MyContet/Blueprints/GM_Craft.GM_Craft_C|GetCodex _gamemode))
  (Utilities|FlowControl|DoOnce false :!label _label
    (:Completed
      (Default|ChangeScene (Variables|Default|GetSound_Mana_Ref))
      (Default|GotoCraft (Variables|/Game/MyContet/Blueprints/GM_Craft.GM_Craft_C|GetCam (Variables|Default|GetGameMode)))
      (Utilities|FlowControl|Sequence
        (:then_0
          (Utilities|FlowControl|DoOnce false
            (:Completed
              (Utilities|FlowControl|Delay 2.5)
              (Default|NextTuto _ui)
              (Default|SetnextDescription _ui)
              (Rendering|Material|SetScalarParameterValue (Variables|/Game/MyContet/Codex/BP_Codex.BP_Codex_C|GetMatTuto _codex) "WeightMask" 1.0 :!class /Script/Engine.MaterialInstanceDynamic)
              (Rendering|Material|SetScalarParameterValue (Variables|Default|GetMatTuto) "WeightMask" 0.0 :!class /Script/Engine.MaterialInstanceDynamic)
              (Default|AllowTutoOpenCodex2 _codex))))
        (:then_1
          (Utilities|FlowControl|Delay 4.0)
          (goto _label Reset))))))

(fn ConstructionScript)