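; BP_BlackHole is a black hole actor that builds a spiral spline and registers itself with the GM_Craft game mode.
; The construction script appends local-space spline points using cosine and sine, stepping the angle by Multi and growing the radius by AdditRadius for each point.
; On BeginPlay, Init casts the game mode to GM_Craft and sets its BlackHole reference to this actor; Tick is empty.
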(event EventBeginPlay
  (CallFunction|Init))

(event Collision|EventActorBeginOverlap
  (params (OtherActor :type Actor%20Object%20Reference)))

(event EventTick
  (params (DeltaSeconds :type Float%20%28single-precision%29)))

(fn ConstructionScript
  (LocalVariables|SetRadius 0.0)
  (for _index (range 0 (LocalVariables|GetSpiralPoints))
    (LocalVariables|SetRadius (+ (LocalVariables|GetRadius) (LocalVariables|GetAdditRadius)))
    (Spline|AddSplinePoint (Variables|Default|GetSpline) (Math|Vector|MakeVector (* (Math|Trig|Cos(Degrees) (* _index (LocalVariables|GetMulti))) (LocalVariables|GetRadius)) (* (LocalVariables|GetRadius) (Math|Trig|Sin(Degrees) (* _index (LocalVariables|GetMulti)))) 0.0) "Local" true)))

(fn Init
  (bind _asgm_craft (Utilities|Casting|CastToGM_Craft (Game|GetGameMode)))
  (Utilities|IsValid _asgm_craft
    (:Is%20Valid
      (bind _output_get (Variables|Default|SetGameMode _asgm_craft))
      (Variables|/Game/MyContet/GM_Craft.GM_Craft_C|SetBlackHole _output_get self))
    (:Is%20Not%20Valid
      (Development|PrintString "GameMode non valide (BP_Crank)"))))