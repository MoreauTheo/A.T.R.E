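; Camera actor that switches between menu, craft and space views using Level Sequences and shows the WB_Camera UI.
; On BeginPlay it registers itself with GM_Craft and places its camera at the start of the AToB spline.
; Space bar, GoToCraft and GoToSpace each play a transition at double speed (GoToCraft in reverse), then immediately set the actor to a hard-coded transform without waiting for the sequence to finish.
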(event EventBeginPlay
  (CallFunction|Init)
  ;[1 1 1] Camera Visuel
  (bind _returnvalue (UserInterface|CreateWidget "/Game/MyContet/Interfaces/Camera/WB_Camera.WB_Camera_C"))
  (Variables|Default|SetUICam _returnvalue)
  (UserInterface|Viewport|AddtoViewport _returnvalue 0))

(event Input|KeyboardEvents|SpaceBar
  (params (Key :type Key%20Structure :default "None"))
  (:Pressed
    (bind _outactor (Sequencer|Player|CreateLevelSequencePlayer (Variables|Default|GetMenuCraft)))
    (Class|MovieSceneSequencePlayer|RestoreState (Variables|/Script/LevelSequence.LevelSequenceActor|GetSequencePlayer _outactor))
    (Components|Timeline|SetPlayRate (Variables|/Script/LevelSequence.LevelSequenceActor|GetSequencePlayer _outactor) 2.0)
    (Sequencer|Player|Play (Variables|/Script/LevelSequence.LevelSequenceActor|GetSequencePlayer _outactor) :!class /Script/MovieScene.MovieSceneSequencePlayer)
    (Transformation|SetActorTransform (Math|Transform|MakeTransform "11.000000,1859.000000,12195.000000" "3.000000,-90.000000,0.000000" "1.000000,1.000000,1.000000"))))

(fn ConstructionScript)

(fn Init
  (bind _asgm_craft (Utilities|Casting|CastToGM_Craft (Game|GetGameMode)))
  (Utilities|IsValid _asgm_craft
    (:Is%20Valid
      (bind _output_get (Variables|Default|SetGameMode _asgm_craft))
      (Variables|/Game/MyContet/Blueprints/GM_Craft.GM_Craft_C|SetCam _output_get self)
      (Transformation|SetWorldLocation (Variables|Default|GetCamera) (.location (Spline|GetTransformatDistanceAlongSpline (Variables|Default|GetAToB) 0.0 "World" false)) false false)
      (Transformation|SetWorldRotation (Variables|Default|GetCamera) (Spline|GetRotationatDistanceAlongSpline (Variables|Default|GetAToB) 0.0 "World") false false))
    (:Is%20Not%20Valid
      (Development|PrintString "GameMode non valide (BP_Cam)"))))

(fn GotoCraft
  (bind _outactor (Sequencer|Player|CreateLevelSequencePlayer (Variables|Default|GetSpaceCraft)))
  (Class|MovieSceneSequencePlayer|RestoreState (Variables|/Script/LevelSequence.LevelSequenceActor|GetSequencePlayer _outactor))
  (Components|Timeline|SetPlayRate (Variables|/Script/LevelSequence.LevelSequenceActor|GetSequencePlayer _outactor) 2.0)
  (Class|MovieSceneSequencePlayer|PlayReverse (Variables|/Script/LevelSequence.LevelSequenceActor|GetSequencePlayer _outactor))
  (Transformation|SetActorTransform (Math|Transform|MakeTransform "11.000000,1859.000000,12195.000000" "3.000000,-90.000000,0.000000" "1.000000,1.000000,1.000000")))

(fn GotoSpace
  (bind _outactor (Sequencer|Player|CreateLevelSequencePlayer (Variables|Default|GetCraftSpace)))
  (Class|MovieSceneSequencePlayer|RestoreState (Variables|/Script/LevelSequence.LevelSequenceActor|GetSequencePlayer _outactor))
  (Components|Timeline|SetPlayRate (Variables|/Script/LevelSequence.LevelSequenceActor|GetSequencePlayer _outactor) 2.0)
  (Sequencer|Player|Play (Variables|/Script/LevelSequence.LevelSequenceActor|GetSequencePlayer _outactor) :!class /Script/MovieScene.MovieSceneSequencePlayer)
  (Transformation|SetActorTransform (Math|Transform|MakeTransform "2858.000000,-3348.000000,13517.000000" "5.600000,-37.000000,0.000000" "1.000000,1.000000,1.000000")))