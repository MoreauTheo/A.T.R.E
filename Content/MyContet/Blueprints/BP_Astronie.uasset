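; BP_Astronie is a body actor for the crafting game mode that registers as the selected body and drives its gauge display.
; Init gets GM_Craft, stores it, sets its SelectedBody to this actor, then sets each gauge actor's Z scale from the matching QuantityJauge entry.
; An invalid game mode reference prints an error, and the event graph and construction script only call their parents.
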(event EventBeginPlay
  (|CallParentFunction))

(event Collision|EventActorBeginOverlap
  (params (OtherActor :type Actor%20Object%20Reference))
  (|CallParentFunction OtherActor) ; This node is disabled and will not be called.\nDrag off pins to build functionality.
)

(event EventTick
  (params (DeltaSeconds :type Float%20%28single-precision%29))
  (|CallParentFunction DeltaSeconds) ; This node is disabled and will not be called.\nDrag off pins to build functionality.
)

(fn ConstructionScript
  (|CallParentFunction))

(fn Init
  (bind _asgm_craft (Utilities|Casting|CastToGM_Craft (Game|GetGameMode)))
  (Utilities|IsValid _asgm_craft
    (:Is%20Valid
      (bind _output_get (Variables|Default|SetGameMode_0 _asgm_craft))
      (Variables|/Game/MyContet/GM_Craft.GM_Craft_C|SetSelectedBody _output_get self)
      (for (_array_element _array_index) (Variables|/Game/MyContet/GM_Craft.GM_Craft_C|GetArrayJauges (Variables|Default|GetGameMode_0))
        (Transformation|SetActorScale3D _array_element (Math|Vector|MakeVector 1.0 1.0 (Utilities|Array|Get(acopy) (Variables|Default|GetQuantityJauge) _array_index)))))
    (:Is%20Not%20Valid
      (Development|PrintString "GameMode non valide (BP_Astronie)"))))