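; Draggable crafting lever that adjusts two gauges and the selected material's quantity in GM_Craft.
; While held, it hides and recenters the cursor, turning vertical mouse movement into clamped pitch.
; Negative-direction movement shifts both gauges' Z scale, updating the material only when both stay between empty and full.
; When released or no material is selected, Tick moves the lever at SpeedReset using LerpRotator.
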(event Input|EnhancedActionEvents|EnhancedInputActionIA_Click
  (params (ActionValue :type Boolean) (ElapsedSeconds :type Float%20%28double-precision%29) (TriggeredSeconds :type Float%20%28double-precision%29) (InputAction :type Input%20Action%20Object%20Reference :default "/Game/MyContet/Inputs/IA_Click.IA_Click"))
  (:Completed
    (Variables|Default|SetLevering false)
    (Variables|/Script/Engine.PlayerController|SetbShowMouseCursor (Game|GetPlayerController 0) true)))

(event EventBeginPlay
  (CallFunction|Init))

(event EventTick
  (params (DeltaSeconds :type Float%20%28single-precision%29))
  (bind _gamemode (Variables|Default|GetGameMode))
  (bind _selectedmaterial (Variables|/Game/MyContet/Blueprints/GM_Craft.GM_Craft_C|GetSelectedMaterial _gamemode))
  (Variables|Default|SetDelta%20Seconds DeltaSeconds)
  (if (Variables|Default|GetLevering)
    (Utilities|IsValid _selectedmaterial
      (:Is%20Valid
        (if (> (Variables|/Game/MyContet/Materiaux/BP_Material.BP_Material_C|GetQuantity _selectedmaterial) 0.0)
          (Class|PlayerController|SetMouseLocation (Game|GetPlayerController 0) 960 540)
          (Variables|Default|SetDeltaMouse (Input|EnhancedActionValues|GetIA_MoveMouse))
          (bind (_rightdirection _changequantity) (CallFunction|Rotate))
          (if (not _rightdirection)
            (CallFunction|ChangesBarres _changequantity _changequantity))))
      (:Is%20Not%20Valid
        (Transformation|SetActorRotation (Math|Rotator|Lerp(Rotator) "-180.000000,0.000000,0.000000" "0, 0, 0" (/ (+ (Variables|Default|GetOldRotation) 1.8e+02) 1.8e+02) true) :!label _label)
        (Variables|Default|SetOldRotation (Math|Float|Clamp(Float) (+ (Variables|Default|GetOldRotation) (* (Variables|Default|GetDelta%20Seconds) (Variables|Default|GetSpeedReset))) -1.8e+02 0.0))))
    (else
      (goto _label))))

(event Collision|EventActorBeginOverlap
  (params (OtherActor :type Actor%20Object%20Reference)))

(event MouseInput|EventActorOnClicked
  (params (ButtonPressed :type Key%20Structure))
  (Variables|Default|SetLevering true)
  (Variables|/Script/Engine.PlayerController|SetbShowMouseCursor (Game|GetPlayerController 0) false))

(fn ConstructionScript)

(fn Init
  (bind _asgm_craft (Utilities|Casting|CastToGM_Craft (Game|GetGameMode)))
  (Utilities|IsValid _asgm_craft
    (:Is%20Valid
      (Variables|Default|SetGameMode _asgm_craft))
    (:Is%20Not%20Valid
      (Development|PrintString "GameMode non valide (BP_Lever)"))))

(fn Rotate
  (bind _deltamouse (Variables|Default|GetDeltaMouse))
  (if (<= (+ (/ (.y _deltamouse) 2.0) (Variables|Default|GetOldRotation)) -1.8e+02)
    (Transformation|SetActorRotation "-180.000000,0.000000,0.000000")
    (elif (>= (+ (/ (.y _deltamouse) 2.0) (Variables|Default|GetOldRotation)) 0.0)
      (Transformation|SetActorRotation "0, 0, 0")
      (else
        (Transformation|SetActorRotation (Math|Rotator|MakeRotator 0.0 (+ (/ (.y _deltamouse) 2.0) (Variables|Default|GetOldRotation)) 0.0))
        (Variables|Default|SetOldRotation (+ (/ (.y _deltamouse) 2.0) (Variables|Default|GetOldRotation)))
        (return (> (.y _deltamouse) 0.0) (.y _deltamouse)))))
  (return false 0.0))

(fn ChangesBarres
  (params (AddJauge1I :type Float%20%28double-precision%29) (AddJauge2I :type Float%20%28double-precision%29))
  (LocalVariables|SetJauge1 (Utilities|Array|Get(acopy) (Variables|/Game/MyContet/Blueprints/GM_Craft.GM_Craft_C|GetArrayJauges (Variables|Default|GetGameMode)) 1))
  (LocalVariables|SetJauge2 (Utilities|Array|Get(acopy) (Variables|/Game/MyContet/Blueprints/GM_Craft.GM_Craft_C|GetArrayJauges (Variables|Default|GetGameMode)) 2))
  (LocalVariables|SetAddJauge1 (/ AddJauge1I 2e+03))
  (bind _result (Math|Float|NegateFloat (/ AddJauge2I 2e+03))
    (:%20%20
      (LocalVariables|SetAdd%20Jauge2 _result)
      (if (> (+ (LocalVariables|GetAddJauge1) (.z (Transformation|GetActorScale3D (LocalVariables|GetJauge1)))) 1.0)
        (Transformation|SetActorScale3D (LocalVariables|GetJauge1) "1.000000,1.000000,1.000000")
        (return)
        (elif (< (+ (LocalVariables|GetAddJauge1) (.z (Transformation|GetActorScale3D (LocalVariables|GetJauge1)))) 0.0)
          (Transformation|SetActorScale3D (LocalVariables|GetJauge1) "1.000000,1.000000,0.000000")
          (return)
          (elif (> (+ (LocalVariables|GetAdd%20Jauge2) (.z (Transformation|GetActorScale3D (LocalVariables|GetJauge2)))) 1.0)
            (Transformation|SetActorScale3D (LocalVariables|GetJauge2) "1.000000,1.000000,1.000000")
            (return)
            (elif (< (+ (LocalVariables|GetAdd%20Jauge2) (.z (Transformation|GetActorScale3D (LocalVariables|GetJauge2)))) 0.0)
              (Transformation|SetActorScale3D (LocalVariables|GetJauge2) "1.000000,1.000000,0.000000")
              (return)
              (else
                (Transformation|SetActorScale3D (LocalVariables|GetJauge2) (Math|Vector|MakeVector 1.0 1.0 (+ (LocalVariables|GetAdd%20Jauge2) (.z (Transformation|GetActorScale3D (LocalVariables|GetJauge2))))))
                (Transformation|SetActorScale3D (LocalVariables|GetJauge1) (Math|Vector|MakeVector 1.0 1.0 (+ (LocalVariables|GetAddJauge1) (.z (Transformation|GetActorScale3D (LocalVariables|GetJauge1))))))
                (Default|UpdateQuantity (Variables|/Game/MyContet/Blueprints/GM_Craft.GM_Craft_C|GetSelectedMaterial (Variables|Default|GetGameMode)) (* (LocalVariables|GetAddJauge1) 5e+01))
                (return)))))))))