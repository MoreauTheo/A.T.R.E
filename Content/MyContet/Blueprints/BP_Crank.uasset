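; Clickable crafting crank that the player turns with the mouse to adjust two gauges using the selected material.
; While held, it centers the hidden cursor and derives yaw from mouse speed and its dot product with a rotating crank vector.
; Negative rotation, with material remaining, shifts the GM_Craft gauges' Z scales within 0–1 and updates material quantity.
; On BeginPlay it also possesses BP_Cam and adds the crafting input context.
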(event Input|EnhancedActionEvents|EnhancedInputActionIA_Click
  (params (ActionValue :type Boolean) (ElapsedSeconds :type Float%20%28double-precision%29) (TriggeredSeconds :type Float%20%28double-precision%29) (InputAction :type Input%20Action%20Object%20Reference :default "/Game/MyContet/Inputs/IA_Click.IA_Click"))
  (:Completed
    (Variables|Default|SetTurning false)
    (Variables|/Script/Engine.PlayerController|SetbShowMouseCursor (Game|GetPlayerController 0) true)))

(event EventBeginPlay
  (CallFunction|Init))

(event EventTick
  (params (DeltaSeconds :type Float%20%28single-precision%29))
  (bind _returnvalue (Input|EnhancedActionValues|GetIA_MoveMouse))
  (bind _gamemode (Variables|Default|GetGameMode))
  (bind _selectedmaterial (Variables|/Game/MyContet/Blueprints/GM_Craft.GM_Craft_C|GetSelectedMaterial _gamemode))
  (if (Variables|Default|GetTurning)
    (Class|PlayerController|SetMouseLocation (Game|GetPlayerController 0) 960 540)
    (Variables|Default|SetDeltaMouse (Math|Vector2D|Normalize2D _returnvalue))
    (bind _rotationvalue (CallFunction|CalculateRotation))
    (bind _output_get (Variables|Default|SetRotation%20Ammount (/ (* _rotationvalue (Math|Vector2D|Vector2DLength _returnvalue)) 3.0)))
    (Transformation|AddLocalRotation (Variables|Default|GetStaticMesh) (Math|Rotator|MakeRotator 0.0 0.0 _output_get) false false)
    (Variables|Default|SetCrankVector (Class|KismetMathLibrary|GetRotated2D (Variables|Default|GetCrankVector) _output_get))
    (if (< _output_get 0.0)
      (Utilities|IsValid _selectedmaterial
        (:Is%20Valid
          (if (> (Variables|/Game/MyContet/Blueprints/Materiaux/BP_Material.BP_Material_C|GetQuantity _selectedmaterial) 0.0)
            (bind _result (Math|Float|NegateFloat (Variables|Default|GetRotation%20Ammount))
              (:%20%20
                (CallFunction|ChangeBarres _result (Variables|Default|GetRotation%20Ammount))))))))))

(event MouseInput|EventActorOnClicked
  (params (ButtonPressed :type Key%20Structure))
  (Variables|Default|SetTurning true)
  (Variables|/Script/Engine.PlayerController|SetbShowMouseCursor (Game|GetPlayerController 0) false))

(fn ConstructionScript)

(fn ChangeBarres
  (params (Barre1%20Add :type Float%20%28double-precision%29) (Barre2%20Add :type Float%20%28double-precision%29))
  (LocalVariables|SetJauge1 (Utilities|Array|Get(acopy) (Variables|/Game/MyContet/Blueprints/GM_Craft.GM_Craft_C|GetArrayJauges (Variables|Default|GetGameMode)) 1))
  (LocalVariables|SetJauge2 (Utilities|Array|Get(acopy) (Variables|/Game/MyContet/Blueprints/GM_Craft.GM_Craft_C|GetArrayJauges (Variables|Default|GetGameMode))))
  (LocalVariables|SetAddJauge1 (/ Barre1%20Add 2e+03))
  (bind _result (Math|Float|NegateFloat (/ Barre2%20Add 2e+03))
    (:%20%20
      (LocalVariables|SetAddJauge2 _result)
      (if (> (+ (LocalVariables|GetAddJauge1) (.z (Transformation|GetActorScale3D (LocalVariables|GetJauge1)))) 1.0)
        (Transformation|SetActorScale3D (LocalVariables|GetJauge1) "1.000000,1.000000,1.000000")
        (return)
        (elif (< (+ (LocalVariables|GetAddJauge1) (.z (Transformation|GetActorScale3D (LocalVariables|GetJauge1)))) 0.0)
          (Transformation|SetActorScale3D (LocalVariables|GetJauge1) "1.000000,1.000000,0.000000")
          (return)
          (elif (> (+ (LocalVariables|GetAddJauge2) (.z (Transformation|GetActorScale3D (LocalVariables|GetJauge2)))) 1.0)
            (Transformation|SetActorScale3D (LocalVariables|GetJauge2) "1.000000,1.000000,1.000000")
            (return)
            (elif (< (+ (LocalVariables|GetAddJauge2) (.z (Transformation|GetActorScale3D (LocalVariables|GetJauge2)))) 0.0)
              (Transformation|SetActorScale3D (LocalVariables|GetJauge2) "1.000000,1.000000,0.000000")
              (return)
              (else
                (Transformation|SetActorScale3D (LocalVariables|GetJauge2) (Math|Vector|MakeVector 1.0 1.0 (+ (LocalVariables|GetAddJauge2) (.z (Transformation|GetActorScale3D (LocalVariables|GetJauge2))))))
                (Transformation|SetActorScale3D (LocalVariables|GetJauge1) (Math|Vector|MakeVector 1.0 1.0 (+ (LocalVariables|GetAddJauge1) (.z (Transformation|GetActorScale3D (LocalVariables|GetJauge1))))))
                (Default|UpdateQuantity (Variables|/Game/MyContet/Blueprints/GM_Craft.GM_Craft_C|GetSelectedMaterial (Variables|Default|GetGameMode)) (/ (- 0.0 (Variables|Default|GetRotation%20Ammount)) 5e+01))
                (return)))))))))

(fn Init
  (bind _asgm_craft (Utilities|Casting|CastToGM_Craft (Game|GetGameMode)))
  (Utilities|IsValid _asgm_craft
    (:Is%20Valid
      (Variables|Default|SetGameMode _asgm_craft)
      (bind _returnvalue (Actor|GetActorOfClass "/Game/MyContet/Blueprints/BP_Cam.BP_Cam_C"))
      (Pawn|Possess (Game|GetPlayerController 0) _returnvalue)
      (Input|AddMappingContext (PlayerController|LocalPlayerSubsystems|GetEnhancedInputLocalPlayerSubsystem (Game|GetPlayerController 0)) "/Game/MyContet/Inputs/IMC_Craft.IMC_Craft" 0 "(bIgnoreAllPressedKeysUntilRelease=True,bForceImmediately=False,bNotifyUserSettings=False)"))
    (:Is%20Not%20Valid
      (Development|PrintString "GameMode non valide (BP_Crank)"))))

(fn CalculateRotation
  (bind _result (Math|Float|NegateFloat (Math|Vector2D|DotProduct(2D) (Math|Vector2D|Normalize2D (Variables|Default|GetCrankVector)) (Math|Vector2D|Normalize2D (Variables|Default|GetDeltaMouse))))
    (:%20%20
      (return _result))))