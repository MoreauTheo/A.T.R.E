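; BP_Material is a clickable material actor for the crafting game mode, showing its quantity on a gauge plane.
; On BeginPlay it creates a dynamic material instance for the plane and caches GM_Craft.
; Clicking it resets the previously selected material's color to white, tints itself green and registers as the game mode's selection.
; UpdateQuantity adds to the quantity, prints it and sends a scaled value to the gauge shader.
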(event EventBeginPlay
  (CallFunction|Init))

(event Collision|EventActorBeginOverlap
  (params (OtherActor :type Actor%20Object%20Reference)))

(event EventTick
  (params (DeltaSeconds :type Float%20%28single-precision%29)))

(event MouseInput|EventActorOnClicked
  (params (ButtonPressed :type Key%20Structure :default "None"))
  (CallFunction|SelectMaterial))

(fn ConstructionScript)

(fn UpdateQuantity
  (params (QuantityAdded :type Float%20%28double-precision%29))
  (bind _output_get (Variables|Default|SetQuantity (+ (Variables|Default|GetQuantity) QuantityAdded)))
  (Development|PrintString (Utilities|String|ToString(Float) _output_get))
  (Rendering|Material|SetScalarParameterValue (Variables|Default|GetMaterialJauge) "QuantityM" (/ (Variables|Default|GetQuantity) 5e+01) :!class /Script/Engine.MaterialInstanceDynamic))

(fn Init
  (bind _returnvalue (Rendering|Material|CreateDynamicMaterialInstance (Variables|Default|GetPlane) 0 "/Game/MyContet/Material/JaugeMateriaux.JaugeMateriaux" "None" :!class /Script/Engine.PrimitiveComponent))
  (Variables|Default|SetMaterialJauge _returnvalue)
  (bind _asgm_craft (Utilities|Casting|CastToGM_Craft (Game|GetGameMode)))
  (Utilities|IsValid _asgm_craft
    (:Is%20Valid
      (Variables|Default|SetGameMode _asgm_craft))
    (:Is%20Not%20Valid
      (Development|PrintString "GameMode non valide (BP_Cam)"))))

(fn SelectMaterial
  (Utilities|IsValid (Variables|/Game/MyContet/Blueprints/GM_Craft.GM_Craft_C|GetSelectedMaterial (Variables|Default|GetGameMode))
    (:Is%20Valid
      (Rendering|Material|SetVectorParameterValue (Variables|BP_Material_C|GetMaterialJauge (Variables|/Game/MyContet/Blueprints/GM_Craft.GM_Craft_C|GetSelectedMaterial (Variables|Default|GetGameMode))) "ColorS" "(R=1.000000,G=1.000000,B=1.000000,A=1.000000)" :!class /Script/Engine.MaterialInstanceDynamic))
    (:Is%20Not%20Valid
      _))
  (Rendering|Material|SetVectorParameterValue (Variables|Default|GetMaterialJauge) "ColorS" "(R=0.168490,G=1.000000,B=0.000000,A=1.000000)" :!class /Script/Engine.MaterialInstanceDynamic)
  (Variables|/Game/MyContet/Blueprints/GM_Craft.GM_Craft_C|SetSelectedMaterial (Variables|Default|GetGameMode) self))