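; Game mode for crafting celestial bodies that orbit a black hole and yield materials.
; SelectBody pays costs from a DataTable-seeded material table, then sets up three scale-driven gauges with two effect zones each.
; ProduceBody converts gauge heights into size, orbit speed, temperature, effects and curve-based material gains, queued in Inventory.
; SpawnBody places the first queued body at its size-indexed black hole slot; StartOrbit runs timed orbiting, after which bodies give materials.
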(event Custom|EndCraftGM
  (Utilities|IsValid (Variables|Default|GetSelectedBody)
    (:Is%20Valid
      (Craft|ProduceBody)
      (Craft|ResetCraft))
    (:Is%20Not%20Valid
      (Development|PrintString "selectinnez un corp"))))

(event EventBeginPlay
  (CallFunction|Init))

(event EventTick
  (params (DeltaSeconds :type Float%20%28single-precision%29))
  (if (Variables|Default|GetOrbiting)
    (Orbit|OrbitBodies)))

(fn ConstructionScript)

(fn SetSectionsSize
  (bind _selectedbody (Variables|Default|GetSelectedBody))
  (bind _selectedbody_2 (Variables|Default|GetSelectedBody))
  (bind _selectedbody_3 (Variables|Default|GetSelectedBody))
  (if (> (Utilities|Array|Length (Variables|Default|GetZones)) 0)
    _
    (else
      (for _index (range 0 5)
        (bind _returnvalue (Game|SpawnActorfromClass "/Game/MyContet/Machines/BP_Section.BP_Section_C" (Math|Transform|MakeTransform "0, 0, 0" "0, 0, 0" "0.000000,0.000000,0.000000") "Undefined" "MultiplyWithRoot" 0 0))
        (Utilities|Array|Add (Variables|Default|GetZones) _returnvalue))))
  (Jauges|SetPairSize (Utilities|Array|Get(acopy) (Variables|Default|GetArrayJauges)) (Variables|/Game/MyContet/Bodies/BP_ParentBodyDataAsset.BP_ParentBodyDataAsset_C|GetBot1 _selectedbody) (Variables|/Game/MyContet/Bodies/BP_ParentBodyDataAsset.BP_ParentBodyDataAsset_C|GetTop1 _selectedbody) (Variables|/Game/MyContet/Bodies/BP_ParentBodyDataAsset.BP_ParentBodyDataAsset_C|GetBot2 _selectedbody) (Variables|/Game/MyContet/Bodies/BP_ParentBodyDataAsset.BP_ParentBodyDataAsset_C|GetTop2 _selectedbody))
  (Jauges|SetPairSize (Utilities|Array|Get(acopy) (Variables|Default|GetArrayJauges) 1) (Variables|/Game/MyContet/Bodies/BP_ParentBodyDataAsset.BP_ParentBodyDataAsset_C|GetBot3 _selectedbody_2) (Variables|/Game/MyContet/Bodies/BP_ParentBodyDataAsset.BP_ParentBodyDataAsset_C|GetTop3 _selectedbody_2) (Variables|/Game/MyContet/Bodies/BP_ParentBodyDataAsset.BP_ParentBodyDataAsset_C|GetBot4 _selectedbody_2) (Variables|/Game/MyContet/Bodies/BP_ParentBodyDataAsset.BP_ParentBodyDataAsset_C|GetTop4 _selectedbody_2) 2)
  (Jauges|SetPairSize (Utilities|Array|Get(acopy) (Variables|Default|GetArrayJauges) 2) (Variables|/Game/MyContet/Bodies/BP_ParentBodyDataAsset.BP_ParentBodyDataAsset_C|GetBot5 _selectedbody_3) (Variables|/Game/MyContet/Bodies/BP_ParentBodyDataAsset.BP_ParentBodyDataAsset_C|GetTop5 _selectedbody_3) (Variables|/Game/MyContet/Bodies/BP_ParentBodyDataAsset.BP_ParentBodyDataAsset_C|GetBot6 _selectedbody_3) (Variables|/Game/MyContet/Bodies/BP_ParentBodyDataAsset.BP_ParentBodyDataAsset_C|GetTop6 _selectedbody_3) 4))

(fn SetPairSize
  (params (Jauge :type BP%20Liquide%20Object%20Reference) (BotZone1 :type Float%20%28double-precision%29) (TopZone1 :type Float%20%28double-precision%29) (BotZone2 :type Float%20%28double-precision%29) (TopZone3 :type Float%20%28double-precision%29) (JaugeIndex :type Integer))
  (bind _returnvalue (Transformation|GetActorLocation Jauge))
  (bind _returnvalue_2 (Transformation|GetActorLocation Jauge))
  (LocalVariables|SetJaugeIndexL JaugeIndex)
  (LocalVariables|SetBotZone1L BotZone1)
  (LocalVariables|SetTopZone1L TopZone1)
  (LocalVariables|SetBotZone2L BotZone2)
  (LocalVariables|SetTopZone2L TopZone3)
  (Transformation|SetActorTransform (Utilities|Array|Get(acopy) (Variables|Default|GetZones) (LocalVariables|GetJaugeIndexL)) (Math|Transform|MakeTransform (Math|Vector|MakeVector (.x _returnvalue) (.y _returnvalue) (+ (.z _returnvalue) (* (* (.z (.BoxExtent (Collision|GetActorBounds Jauge false false))) 2.0) (LocalVariables|GetBotZone1L)))) "0, 0, 0" (Math|Vector|MakeVector 1.0 1.0 (- (LocalVariables|GetTopZone1L) (LocalVariables|GetBotZone1L)))))
  (Transformation|SetActorTransform (Utilities|Array|Get(acopy) (Variables|Default|GetZones) (+ (LocalVariables|GetJaugeIndexL) 1)) (Math|Transform|MakeTransform (Math|Vector|MakeVector (.x _returnvalue_2) (.y _returnvalue_2) (+ (.z _returnvalue_2) (* (* (.z (.BoxExtent (Collision|GetActorBounds Jauge false false))) 2.0) (LocalVariables|GetBotZone2L)))) "0, 0, 0" (Math|Vector|MakeVector 1.0 1.0 (- (LocalVariables|GetTopZone2L) (LocalVariables|GetBotZone2L))))))

(fn CheckforEffect
  (params (Jauge :type BP%20Liquide%20Object%20Reference) (Bot1 :type Float%20%28double-precision%29) (Top1 :type Float%20%28double-precision%29) (Bot2 :type Float%20%28double-precision%29) (Top :type Float%20%28double-precision%29))
  (bind _returnvalue (Transformation|GetActorScale3D Jauge))
  (if (>= (.z _returnvalue) Bot1)
    (if (<= (.z _returnvalue) Top1)
      (return "NewEnumerator1")
      (elif (>= (.z _returnvalue) Bot2)
        (if (<= (.z _returnvalue) Top)
          (return "NewEnumerator2")
          (else
            _)))))
  (return "NewEnumerator0"))

(fn ProduceBody
  (bind _selectedbody (Variables|Default|GetSelectedBody))
  (bind _selectedbody_2 (Variables|Default|GetSelectedBody))
  (bind _selectedbody_3 (Variables|Default|GetSelectedBody))
  (bind _selectedbody_4 (Variables|Default|GetSelectedBody))
  (bind _arrayjauges (Variables|Default|GetArrayJauges))
  (bind _selectedbody_5 (Variables|Default|GetSelectedBody))
  (bind _selectedbody_6 (Variables|Default|GetSelectedBody))
  (bind _output (Utilities|Array|Get(acopy) _arrayjauges 2))
  (bind _curvematerial (Variables|/Game/MyContet/Bodies/BP_ParentBodyDataAsset.BP_ParentBodyDataAsset_C|GetCurveMaterial _selectedbody_5))
  (bind _returnvalue (Transformation|GetActorScale3D _output))
  (bind _returnvalue_2 (Math|Float|Lerp 0.0 1e+02 (.z _returnvalue)))
  (bind _returnvalue_3 (Math|Curves|GetVectorValue _curvematerial _returnvalue_2))
  (Utilities|FlowControl|Sequence
    (:then_0
      ;[0.01692 1 0] Effets
      (bind _newparam (Craft|CheckforEffect (Utilities|Array|Get(acopy) (Variables|Default|GetArrayJauges)) (Variables|/Game/MyContet/Bodies/BP_ParentBodyDataAsset.BP_ParentBodyDataAsset_C|GetBot1 _selectedbody) (Variables|/Game/MyContet/Bodies/BP_ParentBodyDataAsset.BP_ParentBodyDataAsset_C|GetTop1 _selectedbody) (Variables|/Game/MyContet/Bodies/BP_ParentBodyDataAsset.BP_ParentBodyDataAsset_C|GetBot2 _selectedbody) (Variables|/Game/MyContet/Bodies/BP_ParentBodyDataAsset.BP_ParentBodyDataAsset_C|GetTop2 _selectedbody)))
      (LocalVariables|SetEffect1 _newparam))
    (:then_1
      (bind _newparam_2 (Craft|CheckforEffect (Utilities|Array|Get(acopy) (Variables|Default|GetArrayJauges) 1) (Variables|/Game/MyContet/Bodies/BP_ParentBodyDataAsset.BP_ParentBodyDataAsset_C|GetBot3 _selectedbody_3) (Variables|/Game/MyContet/Bodies/BP_ParentBodyDataAsset.BP_ParentBodyDataAsset_C|GetTop3 _selectedbody_3) (Variables|/Game/MyContet/Bodies/BP_ParentBodyDataAsset.BP_ParentBodyDataAsset_C|GetBot4 _selectedbody_3) (Variables|/Game/MyContet/Bodies/BP_ParentBodyDataAsset.BP_ParentBodyDataAsset_C|GetTop4 _selectedbody_3)))
      (LocalVariables|SetEffect2 _newparam_2))
    (:then_2
      (bind _newparam_3 (Craft|CheckforEffect (Utilities|Array|Get(acopy) (Variables|Default|GetArrayJauges) 2) (Variables|/Game/MyContet/Bodies/BP_ParentBodyDataAsset.BP_ParentBodyDataAsset_C|GetBot5 _selectedbody_4) (Variables|/Game/MyContet/Bodies/BP_ParentBodyDataAsset.BP_ParentBodyDataAsset_C|GetTop5 _selectedbody_4) (Variables|/Game/MyContet/Bodies/BP_ParentBodyDataAsset.BP_ParentBodyDataAsset_C|GetBot6 _selectedbody_4) (Variables|/Game/MyContet/Bodies/BP_ParentBodyDataAsset.BP_ParentBodyDataAsset_C|GetTop6 _selectedbody_4)))
      (LocalVariables|SetEffect3 _newparam_3))
    (:then_3
      ;[0.4759 0 1] Tableau Gain Ressource
      (for (_array_element _array_index) (Variables|/Game/MyContet/Bodies/BP_ParentBodyDataAsset.BP_ParentBodyDataAsset_C|GetMaterialGain (Variables|Default|GetSelectedBody))
        (Utilities|Map|Add (LocalVariables|GetTableau) _array_element (Utilities|Array|Get(acopy) (Utilities|Array|MakeArray (.x _returnvalue_3) (.y _returnvalue_3) (.z _returnvalue_3)) _array_index))))
    (:then_4
      ;[0.03215 0.09719 1] Creation Struct
      (Utilities|Array|Add (Variables|Default|GetInventory) (Utilities|Struct|MakeS_CraftedBody (Variables|/Game/MyContet/Bodies/BP_ParentBodyDataAsset.BP_ParentBodyDataAsset_C|GetBodyCrafted (Variables|Default|GetSelectedBody)) (Math|Float|Round (Math|Float|Lerp (Variables|/Game/MyContet/Bodies/BP_ParentBodyDataAsset.BP_ParentBodyDataAsset_C|GetSizeMin _selectedbody_2) (Variables|/Game/MyContet/Bodies/BP_ParentBodyDataAsset.BP_ParentBodyDataAsset_C|GetSizeMax _selectedbody_2) (.z (Transformation|GetActorScale3D (Utilities|Array|Get(acopy) (Variables|Default|GetArrayJauges)))))) (* (Math|Float|Lerp (Variables|/Game/MyContet/Bodies/BP_ParentBodyDataAsset.BP_ParentBodyDataAsset_C|GetSpeedOrbitMin _selectedbody_6) (Variables|/Game/MyContet/Bodies/BP_ParentBodyDataAsset.BP_ParentBodyDataAsset_C|GetSpeedOrbitMax _selectedbody_6) (.z (Transformation|GetActorScale3D (Utilities|Array|Get(acopy) (Variables|Default|GetArrayJauges) 1)))) 4e+03) (Math|Float|Lerp 0.0 1e+02 (.z (Transformation|GetActorScale3D (Utilities|Array|Get(acopy) (Variables|Default|GetArrayJauges) 2)))) (LocalVariables|GetEffect1) (LocalVariables|GetEffect2) (LocalVariables|GetEffect3) (LocalVariables|GetTableau))))))

(fn Init
  (bind _returnvalue (Game|GetPlayerController 0))
  (bind _returnvalue_2 (UserInterface|CreateWidget "/Game/MyContet/Blueprints/Craft_UI.Craft_UI_C" _returnvalue))
  (UserInterface|Viewport|AddtoViewport _returnvalue_2 0)
  (Variables|/Script/Engine.PlayerController|SetbShowMouseCursor _returnvalue true)
  ;[1 1 1] Set MaterialsTable
  (bind _outrownames (DataTable|GetDataTableRowNames (Variables|Materials|GetMaterialDataTable)))
  (for _array_element _outrownames
    (bind _returnvalue_3 (Utilities|GetDataTableRow (Variables|Materials|GetMaterialDataTable) _array_element)
      (:then
        (Utilities|Array|Add (LocalVariables|GetMaterialTypeTable) (.Material (Utilities|Struct|BreakS_MaterialTableBase _returnvalue_3)))
        (Utilities|Array|Add (LocalVariables|GetQuantityTable) (.Quantity (Utilities|Struct|BreakS_MaterialTableBase _returnvalue_3))))))
  (Variables|Materials|SetMaterialsTableEditable (Utilities|Struct|MakeS_MaterialsTable (LocalVariables|GetMaterialTypeTable) (LocalVariables|GetActorsTable) (LocalVariables|GetQuantityTable))))

(fn EndOrbit
  (Variables|Default|SetOrbiting false)
  (for _array_element (Variables|Default|GetPresentBodies)
    (Default|GiveMaterials _array_element)
    (Development|PrintString "Hello")))

(fn OrbitBodies
  (for _array_element (Variables|Default|GetPresentBodies)
    (Default|Orbit _array_element)))

(fn StartOrbit
  (Variables|Default|SetOrbiting true)
  (Utilities|Time|SetTimerbyFunctionName 0 "EndOrbit" 2.0))

(fn SpawnBody
  (if (> (Utilities|Array|Length (Variables|Default|GetInventory)) 0)
    (LocalVariables|SetStructSpawnedBody (Utilities|Array|Get(acopy) (Variables|Default|GetInventory)))
    (bind _returnvalue (Game|SpawnActorfromClass (.bodyclass (LocalVariables|GetStructSpawnedBody)) (Math|Transform|MakeTransform (.location (Transformation|GetWorldTransform (Utilities|Array|Get(acopy) (Variables|/Game/MyContet/Bodies/BlackHole/BP_BlackHole.BP_BlackHole_C|GetPlaces (Variables|Default|GetBlackHole)) (.size (LocalVariables|GetStructSpawnedBody))))) "0, 0, 0" "1.000000,1.000000,1.000000") "AlwaysSpawn" "MultiplyWithRoot" 0 0))
    (LocalVariables|SetSpawnedBody _returnvalue)
    (Utilities|FlowControl|Sequence
      (:then_0
        (Variables|/Game/MyContet/Bodies/BP_BodyCrafted.BP_BodyCrafted_C|SetSize (LocalVariables|GetSpawnedBody) (.size (LocalVariables|GetStructSpawnedBody))))
      (:then_1
        (Variables|/Game/MyContet/Bodies/BP_BodyCrafted.BP_BodyCrafted_C|SetSpeedOrbit (LocalVariables|GetSpawnedBody) (.rotationspeedorbit (LocalVariables|GetStructSpawnedBody))))
      (:then_2
        (Variables|/Game/MyContet/Bodies/BP_BodyCrafted.BP_BodyCrafted_C|SetTemperature (LocalVariables|GetSpawnedBody) (.temperature (LocalVariables|GetStructSpawnedBody))))
      (:then_3
        (Variables|/Game/MyContet/Bodies/BP_BodyCrafted.BP_BodyCrafted_C|SetEffet1 (LocalVariables|GetSpawnedBody) (.effect1 (LocalVariables|GetStructSpawnedBody))))
      (:then_4
        (Variables|/Game/MyContet/Bodies/BP_BodyCrafted.BP_BodyCrafted_C|SetEffet2 (LocalVariables|GetSpawnedBody) (.effect2 (LocalVariables|GetStructSpawnedBody))))
      (:then_5
        (Variables|/Game/MyContet/Bodies/BP_BodyCrafted.BP_BodyCrafted_C|SetEffet3 (LocalVariables|GetSpawnedBody) (.effect3 (LocalVariables|GetStructSpawnedBody))))
      (:then_6
        (Variables|/Game/MyContet/Bodies/BP_BodyCrafted.BP_BodyCrafted_C|SetMaterialGainTab (LocalVariables|GetSpawnedBody) (.gainmaterial (LocalVariables|GetStructSpawnedBody))))
      (:then_7
        (Utilities|Array|RemoveIndex (Variables|Default|GetInventory))
        (Utilities|Array|Add (Variables|Default|GetPresentBodies) (LocalVariables|GetSpawnedBody))
        (Default|Start (LocalVariables|GetSpawnedBody))))))

(fn SelectBody
  (params (ClassBody :type BP%20Parent%20Body%20Data%20Asset%20Object%20Reference))
  (bind _cost (Variables|/Game/MyContet/Bodies/BP_ParentBodyDataAsset.BP_ParentBodyDataAsset_C|GetCost ClassBody))
  (bind _cost_2 (Variables|/Game/MyContet/Bodies/BP_ParentBodyDataAsset.BP_ParentBodyDataAsset_C|GetCost ClassBody))
  ;[1 1 1] Check Quantity To Pay
  (bind _keys (Utilities|Map|Keys _cost_2))
  (bind (_array_element _array_index) (Utilities|Array|ForEachLoopwithBreak _keys)
    (:LoopBody
      (bind _values (Utilities|Map|Values _cost_2))
      (bind _quatity (MaterialsTableOperation|FindRowOfTableEditable _array_element))
      (if (not (>= _quatity (Utilities|Array|Get(acopy) _values _array_index)))
        (LocalVariables|SetEnough false)))
    (:Completed
      (if (LocalVariables|GetEnough)
        (bind _keys_2 (Utilities|Map|Keys _cost))
        (bind (_array_element_2 _array_index_2) (Utilities|Array|ForEachLoopwithBreak _keys_2)
          (:LoopBody
            (bind _values_2 (Utilities|Map|Values _cost))
            (bind _materialtype (MaterialsTableOperation|FindRowOfTableEditable _array_element_2))
            (CallFunction|UpdateQuantity _materialtype (- 0.0 (Utilities|Array|Get(acopy) _values_2 _array_index_2))))
          (:Completed
            (LocalVariables|SetEnough true)
            (Variables|Default|SetSelectedBody ClassBody)
            (for _array_element_3 (Variables|Default|GetArrayJauges)
              (Transformation|SetActorScale3D _array_element_3 (Math|Vector|MakeVector 1.0 1.0 1.0)))
            (Jauges|SetSectionsSize)
            (Jauges|SetJaugeSize)
            (Components|SkeletalMesh|SetSkeletalMeshAsset (Variables|/Game/MyContet/Machines/BP_PreviewPlanet.BP_PreviewPlanet_C|GetSkeletalMesh (Variables|Default|GetPreviewPlanetActor)) (Variables|/Game/MyContet/Bodies/BP_ParentBodyDataAsset.BP_ParentBodyDataAsset_C|GetMesh (Variables|Default|GetSelectedBody)))))))))

(fn SetJaugeSize
  (for (_array_element _array_index) (Variables|Default|GetArrayJauges)
    (Transformation|SetActorScale3D _array_element (Math|Vector|MakeVector 1.0 1.0 (Utilities|Array|Get(acopy) (Variables|/Game/MyContet/Bodies/BP_ParentBodyDataAsset.BP_ParentBodyDataAsset_C|GetQuantityJauge (Variables|Default|GetSelectedBody)) _array_index)))))

(fn ObjectManager
  (bind _returnvalue (Actor|GetActorOfClass "/Script/Engine.PostProcessVolume"))
  (Utilities|IsValid _returnvalue
    (:Is%20Valid
      (Variables|Default|SetMy_PP _returnvalue)
      (for _array_element (Variables|Default|GetArray)
        _))))

(fn FindRow
  (params (Material :type E_Materiaux%20Enum :default "NewEnumerator0"))
  (LocalVariables|SetMaterialL Material)
  (bind _outrownames (DataTable|GetDataTableRowNames (Variables|Materials|GetMaterialDataTable)))
  (for _array_element _outrownames
    (bind _returnvalue (Utilities|GetDataTableRow (Variables|Materials|GetMaterialDataTable) _array_element)
      (:then
        (if (Utilities|Enum|Equal(Enum) (LocalVariables|GetMaterialL) (.Material (Utilities|Struct|BreakS_MaterialTableBase _returnvalue)))
          (return (.Material (Utilities|Struct|BreakS_MaterialTableBase _returnvalue)) (.Actor (Utilities|Struct|BreakS_MaterialTableBase _returnvalue)) (.Quantity (Utilities|Struct|BreakS_MaterialTableBase _returnvalue))))))))

(fn UpdateQuantity
  (params (MaterialType :type E_Materiaux%20Enum :default "NewEnumerator0") (QuantityToAdd :type Float%20%28double-precision%29))
  (bind (_materialtype _actor _index _quatity) (MaterialsTableOperation|FindRowOfTableEditable MaterialType))
  (LocalVariables|SetNewLocalVar_0 _actor)
  (Utilities|Array|SetArrayElem (.Quantity (Utilities|Struct|BreakS_MaterialsTable (Variables|Materials|GetMaterialsTableEditable))) _index (+ _quatity QuantityToAdd))
  (Default|UpdateText (LocalVariables|GetNewLocalVar_0) (+ _quatity QuantityToAdd))
  (Development|PrintString (Utilities|String|ToString(Float) (+ _quatity QuantityToAdd))))

(fn FindRowOfTableEditable
  (params (Material :type E_Materiaux%20Enum :default "NewEnumerator0"))
  (bind _materialstableeditable (Variables|Materials|GetMaterialsTableEditable))
  (bind _returnvalue (Utilities|Array|FindItem (.material _materialstableeditable) Material))
  (if (< _returnvalue 0)
    (Development|PrintString "Materiaux non trouvé")
    (else
      (return (Utilities|Array|Get(acopy) (.material _materialstableeditable) _returnvalue) (Utilities|Array|Get(acopy) (.actor _materialstableeditable) _returnvalue) _returnvalue (Utilities|Array|Get(acopy) (.quantity _materialstableeditable) _returnvalue)))))

(fn ResetCraft
  (Variables|Default|SetSelectedBody 0)
  (for _array_element (Variables|Default|GetArrayJauges)
    (Transformation|SetActorScale3D _array_element "1.000000,1.000000,1.000000")
    (Components|SkeletalMesh|SetSkeletalMeshAsset (Variables|/Game/MyContet/Machines/BP_PreviewPlanet.BP_PreviewPlanet_C|GetSkeletalMesh (Variables|Default|GetPreviewPlanetActor)) 0)))