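; BP_Explosion is a destructible explosion actor that detonates as soon as play begins.
; It crumbles the active clusters of its GCTest geometry collection, then applies a huge constant-falloff radial impulse from that component's location to scatter the pieces.
; It also fades in the explosion sound and spawns the NS_Explosion Niagara effect, then destroys itself on a one-minute timer.
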(event Custom|Sound_Explosion
  (Audio|Components|Audio|FadeIn (Variables|Default|GetSfx_Explosion) 0.3 1.0 0.0 "Linear" :!class /Script/Engine.AudioComponent))

(event EventBeginPlay
  (bind _gc_test (Variables|Default|GetGC_Test))
  (bind _returnvalue (Transformation|GetWorldLocation _gc_test))
  (CallFunction|SoundExplosion)
  (Class|GeometryCollectionComponent|CrumbleActiveClusters _gc_test)
  (Physics|AddRadialImpulse _gc_test _returnvalue 4.5e+16 4.5e+09 "RIF_Constant" false)
  (Niagara|SpawnSystematLocation "/Game/MyContet/VFX/Explosion/NS_Explosion.NS_Explosion" _returnvalue "90.000000,0.000000,0.000000")
  (Utilities|Time|SetTimerbyFunctionName 0 "DestroyActor" 6e+01))

(fn ConstructionScript)

(fn DestroyActor
  (Actor|DestroyActor))