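; BP_RecapCraftScreen is a world actor that hosts the crafting recap panel on a widget component.
; On BeginPlay it creates a WBP_RecapPanel, assigns it to the component, registers both panel and itself with GM_Craft, then hides its whole component hierarchy.
; The K key acts as a debug print, listing the display names of entries in the game mode's editable materials table.
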(event EventBeginPlay
  (CallFunction|Init))

(event Collision|EventActorBeginOverlap
  (params (OtherActor :type Actor%20Object%20Reference)))

(event EventTick
  (params (DeltaSeconds :type Float%20%28single-precision%29)))

(event Input|KeyboardEvents|K
  (params (Key :type Key%20Structure :default "None"))
  (:Pressed
    (for _array_element (.ligne (Variables|/Game/MyContet/Blueprints/GM_Craft.GM_Craft_C|GetMaterialsTableEditable (Variables|Default|GetGameMode)))
      (Development|PrintString (Utilities|GetDisplayName _array_element)))))

(fn ConstructionScript)

(fn Init
  (bind _asgm_craft (Utilities|Casting|CastToGM_Craft (Game|GetGameMode)))
  (Variables|Default|SetGameMode _asgm_craft)
  (bind _returnvalue (Game|ConstructObjectfromClass "/Game/MyContet/RecapCraft/WBP_RecapPanel.WBP_RecapPanel_C"))
  (UserInterface|SetWidget (Variables|Default|GetWidget) _returnvalue)
  (Variables|/Game/MyContet/Blueprints/GM_Craft.GM_Craft_C|SetRecapCraft (Variables|Default|GetGameMode) _returnvalue)
  (Variables|/Game/MyContet/Blueprints/GM_Craft.GM_Craft_C|SetRecapScreen (Variables|Default|GetGameMode) self)
  (Rendering|SetVisibility (Variables|Default|GetDefaultSceneRoot) false true))