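; Crafting manager (GM_Craft) that turns three gauge levels into crafted bodies, based on the recipe read from BP_Astronie.
; On BeginPlay it spawns two scaled BP_Section zones per gauge and sets each gauge's starting Z scale.
; EndCraftGM converts gauge Z scales into size, orbit rotation speed, weight and zone-based effects, then queues the result in Inventory.
; SpawnBody spawns the oldest entry, passing only its effects before calling Start.
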(event Custom|EndCraftGM
  (CallFunction|ProduceBody))

(event EventBeginPlay
  (bind _returnvalue (Actor|GetActorOfClass "/Game/MyContet/Blueprints/BP_Astronie.BP_Astronie_C"))
  (Variables|Default|SetSelectedBody _returnvalue)
  (CallFunction|SpawnSections)
  (CallFunction|Init))

(fn ConstructionScript)

(fn SpawnSections
  (bind _selectedbody (Variables|Default|GetSelectedBody))
  (bind _selectedbody_2 (Variables|Default|GetSelectedBody))
  (bind _selectedbody_3 (Variables|Default|GetSelectedBody))
  (CallFunction|SpawnTwoSection (Utilities|Array|Get(acopy) (Variables|Default|GetArrayJauges)) (Variables|/Game/MyContet/Blueprints/BP_BodyParent.BP_BodyParent_C|GetBot1 _selectedbody_3) (Variables|/Game/MyContet/Blueprints/BP_BodyParent.BP_BodyParent_C|GetTop1 _selectedbody_3) (Variables|/Game/MyContet/Blueprints/BP_BodyParent.BP_BodyParent_C|GetBot2 _selectedbody_3) (Variables|/Game/MyContet/Blueprints/BP_BodyParent.BP_BodyParent_C|GetTop2 _selectedbody_3))
  (CallFunction|SpawnTwoSection (Utilities|Array|Get(acopy) (Variables|Default|GetArrayJauges) 1) (Variables|/Game/MyContet/Blueprints/BP_BodyParent.BP_BodyParent_C|GetBot3 _selectedbody) (Variables|/Game/MyContet/Blueprints/BP_BodyParent.BP_BodyParent_C|GetTop3 _selectedbody) (Variables|/Game/MyContet/Blueprints/BP_BodyParent.BP_BodyParent_C|GetBot4 _selectedbody) (Variables|/Game/MyContet/Blueprints/BP_BodyParent.BP_BodyParent_C|GetTop4 _selectedbody))
  (CallFunction|SpawnTwoSection (Utilities|Array|Get(acopy) (Variables|Default|GetArrayJauges) 2) (Variables|/Game/MyContet/Blueprints/BP_BodyParent.BP_BodyParent_C|GetBot5 _selectedbody_2) (Variables|/Game/MyContet/Blueprints/BP_BodyParent.BP_BodyParent_C|GetTop5 _selectedbody_2) (Variables|/Game/MyContet/Blueprints/BP_BodyParent.BP_BodyParent_C|GetBot6 _selectedbody_2) (Variables|/Game/MyContet/Blueprints/BP_BodyParent.BP_BodyParent_C|GetTop6 _selectedbody_2)))

(fn SpawnTwoSection
  (params (Jauge :type BP%20Liquide%20Object%20Reference) (BotZone1 :type Float%20%28double-precision%29) (TopZone1 :type Float%20%28double-precision%29) (BotZone2 :type Float%20%28double-precision%29) (TopZone3 :type Float%20%28double-precision%29))
  (bind _returnvalue (Transformation|GetActorLocation Jauge))
  (bind _returnvalue_2 (Transformation|GetActorLocation Jauge))
  (LocalVariables|SetBotZone1L BotZone1)
  (LocalVariables|SetTopZone1L TopZone1)
  (LocalVariables|SetBotZone2L BotZone2)
  (LocalVariables|SetTopZone2L TopZone3)
  (Game|SpawnActorfromClass "/Game/MyContet/Blueprints/BP_Section.BP_Section_C" (Math|Transform|MakeTransform (Math|Vector|MakeVector (.x _returnvalue) (.y _returnvalue) (+ (.z _returnvalue) (* (* (.z (.BoxExtent (Collision|GetActorBounds Jauge false false))) 2.0) (LocalVariables|GetBotZone1L)))) "0, 0, 0" (Math|Vector|MakeVector 1.0 1.0 (- (LocalVariables|GetTopZone1L) (LocalVariables|GetBotZone1L)))) "Undefined" "MultiplyWithRoot" 0 0)
  (Game|SpawnActorfromClass "/Game/MyContet/Blueprints/BP_Section.BP_Section_C" (Math|Transform|MakeTransform (Math|Vector|MakeVector (.x _returnvalue_2) (.y _returnvalue_2) (+ (.z _returnvalue_2) (* (* (.z (.BoxExtent (Collision|GetActorBounds Jauge false false))) 2.0) (LocalVariables|GetBotZone2L)))) "0, 0, 0" (Math|Vector|MakeVector 1.0 1.0 (- (LocalVariables|GetTopZone2L) (LocalVariables|GetBotZone2L)))) "Undefined" "MultiplyWithRoot" 0 0))

(fn ProduceBody
  (bind _selectedbody (Variables|Default|GetSelectedBody))
  (bind _arrayjauges (Variables|Default|GetArrayJauges))
  (bind _arrayjauges_2 (Variables|Default|GetArrayJauges))
  (bind _selectedbody_2 (Variables|Default|GetSelectedBody))
  (bind _selectedbody_3 (Variables|Default|GetSelectedBody))
  (bind _arrayjauges_3 (Variables|Default|GetArrayJauges))
  (bind _output (Utilities|Array|Get(acopy) _arrayjauges_2 2))
  (bind _output_2 (Utilities|Array|Get(acopy) _arrayjauges_3))
  (bind _output_3 (Utilities|Array|Get(acopy) _arrayjauges 1))
  (bind _newparam (CallFunction|CheckforEffect _output_2 (Variables|/Game/MyContet/Blueprints/BP_BodyParent.BP_BodyParent_C|GetBot1 _selectedbody_3) (Variables|/Game/MyContet/Blueprints/BP_BodyParent.BP_BodyParent_C|GetTop1 _selectedbody_3) (Variables|/Game/MyContet/Blueprints/BP_BodyParent.BP_BodyParent_C|GetBot2 _selectedbody_3) (Variables|/Game/MyContet/Blueprints/BP_BodyParent.BP_BodyParent_C|GetTop2 _selectedbody_3)))
  (bind _newparam_2 (CallFunction|CheckforEffect _output_3 (Variables|/Game/MyContet/Blueprints/BP_BodyParent.BP_BodyParent_C|GetBot3 _selectedbody) (Variables|/Game/MyContet/Blueprints/BP_BodyParent.BP_BodyParent_C|GetTop3 _selectedbody) (Variables|/Game/MyContet/Blueprints/BP_BodyParent.BP_BodyParent_C|GetBot4 _selectedbody) (Variables|/Game/MyContet/Blueprints/BP_BodyParent.BP_BodyParent_C|GetTop4 _selectedbody)))
  (bind _newparam_3 (CallFunction|CheckforEffect _output (Variables|/Game/MyContet/Blueprints/BP_BodyParent.BP_BodyParent_C|GetBot5 _selectedbody_2) (Variables|/Game/MyContet/Blueprints/BP_BodyParent.BP_BodyParent_C|GetTop5 _selectedbody_2) (Variables|/Game/MyContet/Blueprints/BP_BodyParent.BP_BodyParent_C|GetBot6 _selectedbody_2) (Variables|/Game/MyContet/Blueprints/BP_BodyParent.BP_BodyParent_C|GetTop6 _selectedbody_2)))
  (bind _returnvalue (Utilities|Array|Add (Variables|Default|GetInventory) (Utilities|Struct|MakeS_CraftedBody (Variables|/Game/MyContet/Blueprints/BP_BodyParent.BP_BodyParent_C|GetProductBody (Variables|Default|GetSelectedBody)) (.z (Transformation|GetActorScale3D _output_2)) (.z (Transformation|GetActorScale3D _output_3)) (.z (Transformation|GetActorScale3D _output)) _newparam _newparam_2 _newparam_3)))
  (Development|PrintString (Utilities|String|EnumtoString _newparam_3))
  (Development|PrintString (Utilities|String|EnumtoString _newparam_2))
  (Development|PrintString (Utilities|String|EnumtoString _newparam))
  (Development|PrintString (Utilities|String|ToString(Integer) _returnvalue)))

(fn CheckforEffect
  (params (Jauge :type BP%20Liquide%20Object%20Reference) (Bot1 :type Float%20%28double-precision%29) (Top1 :type Float%20%28double-precision%29) (Bot2 :type Float%20%28double-precision%29) (Top :type Float%20%28double-precision%29))
  (bind _returnvalue (Transformation|GetActorScale3D Jauge))
  (if (>= (.z _returnvalue) Bot1)
    (if (<= (.z _returnvalue) Top1)
      (return "NewEnumerator1")
      (elif (>= (.z _returnvalue) Bot2)
        (if (<= (.z _returnvalue) Top)
          (return "NewEnumerator2")
          (else
            _)))))
  (return "NewEnumerator0"))

(fn SpawnBody
  (bind _inventory (Variables|Default|GetInventory))
  (if (Utilities|Array|IsEmpty _inventory)
    (Development|PrintString "No more body to spawn")
    (else
      (LocalVariables|SetStructCraft (Utilities|Array|Get(acopy) _inventory))
      (bind _returnvalue (Game|SpawnActorfromClass (.bodyclass (LocalVariables|GetStructCraft)) (Math|Transform|MakeTransform "0, 0, 0" "0, 0, 0" "1.000000,1.000000,1.000000") "Undefined" "MultiplyWithRoot" 0 0))
      (LocalVariables|SetCrafted _returnvalue)
      (Utilities|Array|RemoveIndex (Variables|Default|GetInventory))
      (Variables|/Game/MyContet/Blueprints/BP_BodyCrafted.BP_BodyCrafted_C|SetEffet1 (LocalVariables|GetCrafted) (.effect1 (LocalVariables|GetStructCraft)))
      (Variables|/Game/MyContet/Blueprints/BP_BodyCrafted.BP_BodyCrafted_C|SetEffet2 (LocalVariables|GetCrafted) (.effect2 (LocalVariables|GetStructCraft)))
      (Variables|/Game/MyContet/Blueprints/BP_BodyCrafted.BP_BodyCrafted_C|SetEffet3 (LocalVariables|GetCrafted) (.effect3 (LocalVariables|GetStructCraft)))
      (Default|Start (LocalVariables|GetCrafted)))))

(fn Init
  (for (_array_element _array_index) (Variables|Default|GetArrayJauges)
    (Transformation|SetActorScale3D _array_element (Math|Vector|MakeVector 1.0 1.0 (Utilities|Array|Get(acopy) (Variables|/Game/MyContet/Blueprints/BP_BodyParent.BP_BodyParent_C|GetQuantityJauge (Variables|Default|GetSelectedBody)) _array_index)))))