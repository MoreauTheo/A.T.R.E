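; Clickable crafting-material actor that shows the available quantity of its material type on a widget.
; Shortly after BeginPlay, it caches GM_Craft, registers itself in that game mode's editable materials table and displays the stored quantity.
; Clicking it updates the craft screen image and has the game mode decrement the quantity; cursor hover turns MaterialWheel each Tick.
; SelectMaterial can set the game mode's selected material, but nothing here calls it.
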(event EventBeginPlay
  (Utilities|FlowControl|Delay 0.2)
  (CallFunction|Init))

(event EventTick
  (params (DeltaSeconds :type Float%20%28single-precision%29))
  (if (Variables|Default|GetHovered)
    (Default|Turn (Variables|Default|GetMaterialWheel))))

(event MouseInput|EventActorOnClicked
  (params (ButtonPressed :type Key%20Structure :default "None"))
  (Default|ChangeImage (Variables|/Game/MyContet/Blueprints/GM_Craft.GM_Craft_C|GetCraftScreen (Variables|Default|GetGameMode)) (Variables|Default|GetSelectionTexture))
  (Default|UpdateQuantity (Variables|Default|GetGameMode) (Variables|Default|GetMaterialType) -1))

(event MouseInput|EventActorBeginCursorOver
  (Variables|Default|SetHovered true))

(event MouseInput|EventActorEndCursorOver
  (Variables|Default|SetHovered false))

(fn ConstructionScript)

(fn Init
  (bind _asgm_craft (Utilities|Casting|CastToGM_Craft (Game|GetGameMode)))
  (Utilities|IsValid _asgm_craft
    (:Is%20Valid
      (bind _output_get (Variables|Default|SetGameMode _asgm_craft))
      (bind (_materialtype _actor _index _quatity) (Default|FindRowOfTableEditable _output_get (Variables|Default|GetMaterialType)))
      (Utilities|Array|SetArrayElem (.Actor (Utilities|Struct|BreakS_MaterialsTable (Variables|/Game/MyContet/Blueprints/GM_Craft.GM_Craft_C|GetMaterialsTableEditable (Variables|Default|GetGameMode)))) _index self true)
      (bind _asbp_material_quantity_display (Utilities|Casting|CastToBP_MaterialQuantityDisplay (UserInterface|GetWidget (Variables|Default|GetWidget))))
      (Variables|Default|SetDisplayQuantity _asbp_material_quantity_display)
      (Development|PrintString (Utilities|String|ToString(Integer) _quatity))
      (CallFunction|UpdateText _quatity))
    (:Is%20Not%20Valid
      (Development|PrintString "GameMode non valide (BP_Cam)"))))

(fn SelectMaterial
  (bind _output_get (Variables|/Game/MyContet/Blueprints/GM_Craft.GM_Craft_C|SetSelectedMaterial (Variables|Default|GetGameMode) (Variables|Default|GetMaterialType)))
  (Development|PrintString (Utilities|String|EnumtoString _output_get)))

(fn UpdateText
  (params (Number :type Integer))
  (Variables|/Script/UMG.TextBlock|SetText (Variables|/Game/MyContet/Materiaux/BP_MaterialQuantityDisplay.BP_MaterialQuantityDisplay_C|GetTextQuantity (Variables|Default|GetDisplayQuantity)) (Utilities|Text|ToText(Integer) Number)))