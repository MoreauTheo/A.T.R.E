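; Bp_Cinematic is an actor that times a simple three-step sequence of planes and text, likely slides in a cinematic.
; On BeginPlay it waits through chained five-second delays, destroying each plane and text component pair in turn.
; The construction script is empty, and nothing happens after the third pair is removed.
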(event EventBeginPlay
  (Utilities|FlowControl|Delay 5.0)
  (Components|DestroyComponent (Variables|Default|GetPlan1))
  (Utilities|FlowControl|Delay 5.0)
  (Components|DestroyComponent (Variables|Default|GetPlane2))
  (Utilities|FlowControl|Delay 5.0)
  (Components|DestroyComponent (Variables|Default|GetPlane3)))

(fn ConstructionScript)