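; BP_L1 is a clickable tutorial actor with a highlighted Tube and a Material component that spins continuously.
; Clicks pass through DoOnce gates, re-armed by Allow events, that advance the GameMode UI tutorial.
; Steps clear the highlight through a dynamic material's WeightMask, hand the highlight to BP_Crank or open the BP_Button_Craft gate.
; The last gate re-arms from the preceding step and is sequenced first, so it waits for another click.
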(event Custom|Click
  (bind _gamemode (Variables|Default|GetGameMode))
  (bind _gamemode_2 (Variables|Default|GetGameMode))
  (bind _gamemode_3 (Variables|Default|GetGameMode))
  (bind _ui (Variables|/Game/MyContet/Blueprints/GM_Craft.GM_Craft_C|GetUI _gamemode))
  (bind _ui_2 (Variables|/Game/MyContet/Blueprints/GM_Craft.GM_Craft_C|GetUI _gamemode_2))
  (bind _ui_3 (Variables|/Game/MyContet/Blueprints/GM_Craft.GM_Craft_C|GetUI _gamemode_3))
  (Utilities|FlowControl|Sequence
    (:then_0
      (Utilities|FlowControl|DoOnce true
        (:Completed
          (Default|NextTuto _ui)
          (Default|SetnextDescription _ui)
          (Rendering|Material|SetScalarParameterValue (Variables|Default|GetMaterialTuto) "WeightMask" 0.0 :!class /Script/Engine.MaterialInstanceDynamic)
          (bind _returnvalue (Actor|GetActorOfClass "/Game/MyContet/Machines/BP_Button_Craft.BP_Button_Craft_C"))
          (Default|OpenGateButton _returnvalue))))
    (:then_1
      (Utilities|FlowControl|DoOnce true
        (:Completed
          (Rendering|Material|SetScalarParameterValue (Variables|Default|GetMaterialTuto) "WeightMask" 0.0 :!class /Script/Engine.MaterialInstanceDynamic)
          (bind _returnvalue_2 (Actor|GetActorOfClass "/Game/MyContet/Machines/BP_Crank.BP_Crank_C"))
          (Default|AllowTutoCrank _returnvalue_2)
          (Rendering|Material|SetScalarParameterValue (Variables|/Game/MyContet/Machines/BP_Crank.BP_Crank_C|GetMatTuto _returnvalue_2) "WeightMask" 1.0 :!class /Script/Engine.MaterialInstanceDynamic)
          (Default|NextTuto _ui_2)
          (Default|SetnextDescription _ui_2))))
    (:then_2
      (Utilities|FlowControl|DoOnce true
        (:Completed
          (Default|NextTuto _ui_3)
          (Default|SetnextDescription _ui_3)
          (CallFunction|AllowTuto3))))))

(event Custom|AllowTutoL1
  (bind _gamemode (Variables|Default|GetGameMode))
  (bind _ui (Variables|/Game/MyContet/Blueprints/GM_Craft.GM_Craft_C|GetUI _gamemode))
  (Utilities|FlowControl|DoOnce true) ; enters at Reset
)

(event Custom|AllowTuto3
  (bind _gamemode (Variables|Default|GetGameMode))
  (bind _ui (Variables|/Game/MyContet/Blueprints/GM_Craft.GM_Craft_C|GetUI _gamemode))
  (Utilities|FlowControl|DoOnce true) ; enters at Reset
)

(event Custom|AllowTuto2
  (bind _gamemode (Variables|Default|GetGameMode))
  (bind _ui (Variables|/Game/MyContet/Blueprints/GM_Craft.GM_Craft_C|GetUI _gamemode))
  (Utilities|FlowControl|DoOnce true) ; enters at Reset
)

(event EventBeginPlay
  (|CallParentFunction)
  (bind _returnvalue (Rendering|Material|CreateDynamicMaterialInstance "/Game/MyContet/Materials/M_HighlighBox.M_HighlighBox" "None" "None" :!class /Script/Engine.KismetMaterialLibrary))
  (bind _output_get (Variables|Default|SetMaterialTuto _returnvalue))
  (Rendering|Material|SetMaterial (Variables|Default|GetTube) 1 _output_get))

(event Collision|EventActorBeginOverlap
  (params (OtherActor :type Actor%20Object%20Reference)))

(event EventTick
  (params (DeltaSeconds :type Float%20%28single-precision%29))
  (bind _material (Variables|Default|GetMaterial))
  (|CallParentFunction DeltaSeconds)
  (Transformation|AddLocalRotation _material (Math|Rotator|MakeRotator 0.0 (* (Variables|Default|GetRotationYSpeed) DeltaSeconds) 0.0) false false)
  (Transformation|AddLocalRotation _material (Math|Rotator|MakeRotator 0.0 0.0 (* (Variables|Default|GetRotationZSpeed) DeltaSeconds)) false false))

(fn ConstructionScript
  (|CallParentFunction))

(fn ChangeMatTuto
  (params (Weight :type Float%20%28double-precision%29))
  (Rendering|Material|SetScalarParameterValue (Variables|Default|GetMaterialTuto) "WeightMask" Weight :!class /Script/Engine.MaterialInstanceDynamic))

(fn Clicked
  (|CallParentFunction)
  (CallFunction|Click))