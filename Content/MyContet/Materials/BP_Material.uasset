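; Clickable material capsule in the crafting scene that spends one unit and applies its selection texture to the craft screen.
; Registers itself in GM_Craft's material table, which supplies unlock state and quantity.
; Hovering turns the material wheel and sets a lock-aware cursor; clicking checks body and stock, flashes the light and offsets rotation from the crank.
; Size functions swap between three texture variants, and Unlock reveals the glass tube and light.
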(event EventBeginPlay
  (Utilities|FlowControl|Delay 0.2)
  (CallFunction|Init))

(event EventTick
  (params (DeltaSeconds :type Float%20%28single-precision%29))
  (if (Variables|Default|GetHovered)
    (Default|Turn (Variables|Default|GetMaterialWheel))))

(event MouseInput|EventActorOnClicked
  (params (ButtonPressed :type Key%20Structure))
  (CallFunction|Clicked)
  ;[1 1 1] Material Selection Feedback
  (Rendering|Components|Light|SetIntensity (Variables|Default|GetPointLight) 1e+01)
  (bind _newtrack_0 (Timeline|LightFading PlayFromStart)
    (:Update
      (Rendering|Components|Light|SetIntensity (Variables|Default|GetPointLight) _newtrack_0))))

(event MouseInput|EventActorBeginCursorOver
  (bind _returnvalue (Game|GetPlayerController 0))
  (Variables|Default|SetHovered true)
  (bind _unlocked (Default|FindRowOfTableEditable (Variables|Default|GetGameMode) (Variables|Default|GetMaterialType)))
  (if _unlocked
    (Variables|/Script/Engine.PlayerController|SetCurrentMouseCursor _returnvalue "ResizeLeftRight")
    (else
      (Variables|/Script/Engine.PlayerController|SetCurrentMouseCursor _returnvalue "SlashedCircle"))))

(event MouseInput|EventActorEndCursorOver
  (Variables|Default|SetHovered false)
  (Variables|/Script/Engine.PlayerController|SetCurrentMouseCursor (Game|GetPlayerController 0) "Default"))

(fn ConstructionScript)

(fn Init
  (bind _asgm_craft (Utilities|Casting|CastToGM_Craft (Game|GetGameMode)))
  (Utilities|IsValid _asgm_craft
    (:Is%20Valid
      (bind _output_get (Variables|Default|SetGameMode _asgm_craft))
      (bind _returnvalue (Actor|GetActorOfClass "/Game/MyContet/Sound/Bp_Sound_Manager.Bp_Sound_Manager_C"))
      (Variables|Default|SetSound_Mana_Ref _returnvalue)
      ;[1 1 1] Je mettais des sons et cela a commencé à bug pour la rotation de la mats wheel donc j'ai ajouté que cela et ça marche
      (bind _returnvalue_2 (Actor|GetActorOfClass "/Game/MyContet/MaterialWheel/BP_MaterialWheel.BP_MaterialWheel_C"))
      (Variables|Default|SetMaterialWheel _returnvalue_2)
      (bind (_materialtype _actor _index _quatity) (Default|FindRowOfTableEditable _output_get (Variables|Default|GetMaterialType)))
      (Utilities|Array|SetArrayElem (.Actor (Utilities|Struct|BreakS_MaterialsTable (Variables|/Game/MyContet/Blueprints/GM_Craft.GM_Craft_C|GetMaterialsTableEditable (Variables|Default|GetGameMode)))) _index self true)
      (bind _asbp_material_quantity_display (Utilities|Casting|CastToBP_MaterialQuantityDisplay (UserInterface|GetWidget (Variables|Default|GetWidget))))
      (Variables|Default|SetDisplayQuantity _asbp_material_quantity_display)
      (CallFunction|UpdateText _quatity))
    (:Is%20Not%20Valid
      (Development|PrintString "GameMode non valide (BP_Cam)"))))

(fn SelectMaterial
  (bind _output_get (Variables|/Game/MyContet/Blueprints/GM_Craft.GM_Craft_C|SetSelectedMaterial (Variables|Default|GetGameMode) (Variables|Default|GetMaterialType)))
  (Development|PrintString (Utilities|String|EnumtoString _output_get)))

(fn UpdateText
  (params (Number :type Integer))
  (Variables|/Script/UMG.TextBlock|SetText (Variables|/Game/MyContet/Materials/BP_MaterialQuantityDisplay.BP_MaterialQuantityDisplay_C|GetTextQuantity (Variables|Default|GetDisplayQuantity)) (Utilities|Text|ToText(Integer) Number)))

(fn SizeUp
  (if (!= (Variables|Default|GetIndexArea) 2)
    (if (Utilities|Enum|NotEqual(Enum) (Variables|Default|GetMaterialType) "NewEnumerator3")
      (bind _quatity (Default|FindRowOfTableEditable (Variables|Default|GetGameMode) (Variables|Default|GetMaterialType)))
      (if (> _quatity 0)
        (if (< (+ (Variables|Default|GetIndexArea) 1) (Utilities|Array|Length (Variables|Default|GetSelectionTextures)))
          (Variables|Default|SetIndexArea 2)
          (Default|ChangeImage (Variables|/Game/MyContet/Blueprints/GM_Craft.GM_Craft_C|GetCraftScreen (Variables|Default|GetGameMode)) (Utilities|Array|Get(acopy) (Variables|Default|GetSelectionTextures) (Variables|Default|GetIndexArea)))
          (Default|SizeUpSound (Variables|Default|GetSound_Mana_Ref))
          (else
            (Development|PrintString "NotEnoughTextures")
            (Default|WarningMatsBody (Variables|/Game/MyContet/Blueprints/BP_Cam.BP_Cam_C|GetUICam (Variables|/Game/MyContet/Blueprints/GM_Craft.GM_Craft_C|GetCam (Variables|Default|GetGameMode))) "NewEnumerator6")))))))

(fn SizeDown
  (if (!= (Variables|Default|GetIndexArea) 0)
    (if (Utilities|Enum|NotEqual(Enum) (Variables|Default|GetMaterialType) "NewEnumerator3")
      (if (>= (- (Variables|Default|GetIndexArea) 1) 0)
        (Variables|Default|SetIndexArea 0)
        (Default|ChangeImage (Variables|/Game/MyContet/Blueprints/GM_Craft.GM_Craft_C|GetCraftScreen (Variables|Default|GetGameMode)) (Utilities|Array|Get(acopy) (Variables|Default|GetSelectionTextures) (Variables|Default|GetIndexArea)))
        (Default|SizeDownSound (Variables|Default|GetSound_Mana_Ref))
        (else
          (Development|PrintString "NotEnoughTextures")
          (Default|WarningMatsBody (Variables|/Game/MyContet/Blueprints/BP_Cam.BP_Cam_C|GetUICam (Variables|/Game/MyContet/Blueprints/GM_Craft.GM_Craft_C|GetCam (Variables|Default|GetGameMode))) "NewEnumerator5"))))))

(fn Clicked
  (bind _gamemode (Variables|Default|GetGameMode))
  (bind _cam (Variables|/Game/MyContet/Blueprints/GM_Craft.GM_Craft_C|GetCam _gamemode))
  (bind _uicam (Variables|/Game/MyContet/Blueprints/BP_Cam.BP_Cam_C|GetUICam _cam))
  (bind _isselected (Default|CheckifBodySelected _gamemode "Veuillez selectionner un corps"))
  (if _isselected
    (bind _quatity (Default|FindRowOfTableEditable (Variables|Default|GetGameMode) (Variables|Default|GetMaterialType)))
    (if (> _quatity 0)
      (Default|UseMats (Variables|Default|GetSound_Mana_Ref))
      (Variables|Default|SetIndexArea 0)
      (Default|ConfirmPose (Variables|/Game/MyContet/Blueprints/GM_Craft.GM_Craft_C|GetCraftScreen (Variables|Default|GetGameMode)))
      (Default|ChangeImage (Variables|/Game/MyContet/Blueprints/GM_Craft.GM_Craft_C|GetCraftScreen (Variables|Default|GetGameMode)) (Utilities|Array|Get(acopy) (Variables|Default|GetSelectionTextures) (Variables|Default|GetIndexArea)))
      (Default|UpdateQuantity (Variables|Default|GetGameMode) (Variables|Default|GetMaterialType) -1)
      (Variables|/Game/MyContet/Blueprints/GM_Craft.GM_Craft_C|SetMaterialSelected (Variables|Default|GetGameMode) self)
      (bind _returnvalue (Actor|GetActorOfClass "/Game/MyContet/Machines/BP_Crank.BP_Crank_C"))
      (bind _output_get (Variables|/Game/MyContet/Machines/BP_Crank.BP_Crank_C|SetCurrentRotation _returnvalue (+ (Variables|/Game/MyContet/Machines/BP_Crank.BP_Crank_C|GetCurrentRotation _returnvalue) 9e+01)))
      (Rendering|Material|SetScalarParameterValue (Variables|/Game/MyContet/Craft2/BP_CraftScreen.BP_CraftScreen_C|GetMaterial%20Rotaion (Variables|/Game/MyContet/Blueprints/GM_Craft.GM_Craft_C|GetCraftScreen (Variables|Default|GetGameMode))) "RotationAmmount" (/ _output_get 1e+02) :!class /Script/Engine.MaterialInstanceDynamic)
      (else
        (Development|PrintString "La capsule est vide.")
        (Default|WarningMatsBody _uicam "NewEnumerator4")))
    (else
      (Default|WarningMatsBody _uicam "NewEnumerator1"))))

(fn Unlock
  (Rendering|Material|SetMaterial (Variables|Default|GetTube) 0 "/Game/MyContet/Mesh/M_Glass.M_Glass")
  (Rendering|SetVisibility (Variables|Default|GetCube1) true false)
  (Rendering|SetVisibility (Variables|Default|GetPointLight) true false))

(fn SizeMiddle
  (if (!= (Variables|Default|GetIndexArea) 1)
    (if (Utilities|Enum|NotEqual(Enum) (Variables|Default|GetMaterialType) "NewEnumerator3")
      (Variables|Default|SetIndexArea 1)
      (Default|ChangeImage (Variables|/Game/MyContet/Blueprints/GM_Craft.GM_Craft_C|GetCraftScreen (Variables|Default|GetGameMode)) (Utilities|Array|Get(acopy) (Variables|Default|GetSelectionTextures) (Variables|Default|GetIndexArea))))))