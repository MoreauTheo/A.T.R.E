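; BP_StarLifetime is a child star that modifies the lifetime of the crafted body by its AddLifetime value.
; At BeginPlay the sphere gets the good heart material for a positive value, otherwise the bad one.
; StarEffect adds the value to SCraftedBody.Lifetime on the GameMode, and SetOverText shows it in the tooltip as "tours".
; When the parent's SetSelected returns true, selection adds or subtracts it from NumberTurn and refreshes the recap.
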(event EventBeginPlay
  (|CallParentFunction)
  (if (> (Variables|Default|GetAddLifetime) 0)
    (Rendering|Material|SetMaterial (Variables|Default|GetSphere) 0 "/Game/MyContet/Craft2/Stars/Heart/M_Heart_Good.M_Heart_Good")
    (else
      (Rendering|Material|SetMaterial (Variables|Default|GetSphere) 0 "/Game/MyContet/Craft2/Stars/Heart/M_Heart_Bad.M_Heart_Bad"))))

(event Collision|EventActorBeginOverlap
  (params (OtherActor :type Actor%20Object%20Reference))
  (|CallParentFunction OtherActor) ; This node is disabled and will not be called.\nDrag off pins to build functionality.
)

(event EventTick
  (params (DeltaSeconds :type Float%20%28single-precision%29))
  (|CallParentFunction DeltaSeconds) ; This node is disabled and will not be called.\nDrag off pins to build functionality.
)

(fn ConstructionScript
  (|CallParentFunction))

(fn StarEffect
  (bind _gamemode (Variables|Default|GetGameMode))
  (Variables|/Game/MyContet/Blueprints/GM_Craft.GM_Craft_C|SetS%20Crafted%20Body _gamemode (Utilities|Struct|MakeS_CraftedBody (.name (Variables|/Game/MyContet/Blueprints/GM_Craft.GM_Craft_C|GetS%20Crafted%20Body _gamemode)) (.bodyclass (Variables|/Game/MyContet/Blueprints/GM_Craft.GM_Craft_C|GetS%20Crafted%20Body _gamemode)) (.gainmaterial (Variables|/Game/MyContet/Blueprints/GM_Craft.GM_Craft_C|GetS%20Crafted%20Body _gamemode)) (+ (.lifetime (Variables|/Game/MyContet/Blueprints/GM_Craft.GM_Craft_C|GetS%20Crafted%20Body _gamemode)) (Variables|Default|GetAddLifetime))))
  (|CallParentFunction))

(fn SetOverText
  (|CallParentFunction)
  (Variables|/Script/UMG.TextBlock|SetText (Variables|/Game/MyContet/Blueprints/GM_Craft.GM_Craft_C|GetTextTooltipStar (Variables|Default|GetGameMode)) (Utilities|Text|ToText(String) (Utilities|String|Append (Utilities|String|ToString(Integer) (Variables|Default|GetAddLifetime)) " tours"))))

(fn SetSelected
  (params (IsSelected :type Boolean))
  (bind _gamemode (Variables|Default|GetGameMode))
  (bind _gamemode_2 (Variables|Default|GetGameMode))
  (bind _newparam (|CallParentFunction IsSelected))
  (if _newparam
    (if IsSelected
      (Variables|/Game/MyContet/Blueprints/GM_Craft.GM_Craft_C|SetNumberTurn _gamemode_2 (+ (Variables|/Game/MyContet/Blueprints/GM_Craft.GM_Craft_C|GetNumberTurn _gamemode_2) (Variables|Default|GetAddLifetime)))
      (else
        (Variables|/Game/MyContet/Blueprints/GM_Craft.GM_Craft_C|SetNumberTurn _gamemode (- (Variables|/Game/MyContet/Blueprints/GM_Craft.GM_Craft_C|GetNumberTurn _gamemode) (Variables|Default|GetAddLifetime)))))
    (Default|SetRecap (Variables|Default|GetGameMode))))