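; BP_StarMat is a crafting star that adds or subtracts material amounts, held in its MatiarlsAdded map, and shows a good or bad sphere material by the first amount's sign.
; StarEffect merges the map into the GameMode crafted body's GainMaterial totals.
; Hover text shows the first entry's amount and table icon.
; Selection changes adjust the GameMode's RecapMaterial, returning after the first key, and refresh the recap.
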(event EventBeginPlay
  (|CallParentFunction)
  (bind _values (Utilities|Map|Values (Variables|Default|GetMatiarlsAdded)))
  (if (> (Utilities|Array|Get(acopy) _values) 0)
    (Rendering|Material|SetMaterial (Variables|Default|GetSphere) 0 "/Game/MyContet/Craft2/Stars/Star/M_Star_Good.M_Star_Good")
    (else
      (Rendering|Material|SetMaterial (Variables|Default|GetSphere) 0 "/Game/MyContet/Craft2/Stars/Star/M_Star_Bad.M_Star_Bad"))))

(event Collision|EventActorBeginOverlap
  (params (OtherActor :type Actor%20Object%20Reference))
  (|CallParentFunction OtherActor) ; This node is disabled and will not be called.\nDrag off pins to build functionality.
)

(event EventTick
  (params (DeltaSeconds :type Float%20%28single-precision%29))
  (|CallParentFunction DeltaSeconds) ; This node is disabled and will not be called.\nDrag off pins to build functionality.
)

(fn ConstructionScript
  (|CallParentFunction))

(fn StarEffect
  (bind _matiarlsadded (Variables|Default|GetMatiarlsAdded))
  (bind _keys (Utilities|Map|Keys _matiarlsadded))
  (bind _values (Utilities|Map|Values _matiarlsadded))
  (for (_array_element _array_index) _keys
    (if (.ReturnValue (Utilities|Map|Find (.gainmaterial (Variables|/Game/MyContet/Blueprints/GM_Craft.GM_Craft_C|GetS%20Crafted%20Body (Variables|Default|GetGameMode))) _array_element))
      (Utilities|Map|Add (.gainmaterial (Variables|/Game/MyContet/Blueprints/GM_Craft.GM_Craft_C|GetS%20Crafted%20Body (Variables|Default|GetGameMode))) _array_element (+ (.Value (Utilities|Map|Find (.gainmaterial (Variables|/Game/MyContet/Blueprints/GM_Craft.GM_Craft_C|GetS%20Crafted%20Body (Variables|Default|GetGameMode))) _array_element)) (Utilities|Array|Get(acopy) _values _array_index)))
      (else
        (Utilities|Map|Add (.gainmaterial (Variables|/Game/MyContet/Blueprints/GM_Craft.GM_Craft_C|GetS%20Crafted%20Body (Variables|Default|GetGameMode))) _array_element (Utilities|Array|Get(acopy) _values _array_index)))))
  (|CallParentFunction))

(fn SetOverText
  (bind _matiarlsadded (Variables|Default|GetMatiarlsAdded))
  (|CallParentFunction)
  (bind _values (Utilities|Map|Values _matiarlsadded))
  (bind _keys (Utilities|Map|Keys _matiarlsadded))
  (Variables|/Script/UMG.TextBlock|SetText (Variables|/Game/MyContet/Blueprints/GM_Craft.GM_Craft_C|GetTextTooltipStar (Variables|Default|GetGameMode)) (Utilities|Text|ToText(String) (Utilities|String|Append (Utilities|String|ToString(Integer) (Utilities|Array|Get(acopy) _values)) " ")))
  (bind _actor (Default|FindRowOfTableEditable (Variables|Default|GetGameMode) (Utilities|Array|Get(acopy) _keys)))
  (Appearance|SetBrushfromTexture (Variables|/Game/MyContet/Blueprints/Craft_UI.Craft_UI_C|GetIconMaterial (Variables|/Game/MyContet/Blueprints/GM_Craft.GM_Craft_C|GetUI (Variables|Default|GetGameMode))) (Variables|/Game/MyContet/Materials/BP_Material.BP_Material_C|GetSelectionTexture _actor) false))

(fn SetSelected
  (params (IsSelected :type Boolean))
  (bind _gamemode (Variables|Default|GetGameMode))
  (bind _matiarlsadded (Variables|Default|GetMatiarlsAdded))
  (bind _gamemode_2 (Variables|Default|GetGameMode))
  (bind _matiarlsadded_2 (Variables|Default|GetMatiarlsAdded))
  (bind _recapmaterial (Variables|/Game/MyContet/Blueprints/GM_Craft.GM_Craft_C|GetRecapMaterial _gamemode))
  (bind _recapmaterial_2 (Variables|/Game/MyContet/Blueprints/GM_Craft.GM_Craft_C|GetRecapMaterial _gamemode_2))
  (bind _newparam (|CallParentFunction IsSelected))
  (if _newparam
    (if (Variables|Default|GetSelected)
      (bind _keys (Utilities|Map|Keys _matiarlsadded_2))
      (for _array_element _keys
        (Utilities|Map|Add _recapmaterial_2 _array_element (+ (.Value (Utilities|Map|Find _matiarlsadded_2 _array_element)) (.Value (Utilities|Map|Find _recapmaterial_2 _array_element))))
        (Default|SetRecap (Variables|Default|GetGameMode))
        (return (LocalVariables|GetNewLocalVar)))
      (else
        (bind _keys_2 (Utilities|Map|Keys _matiarlsadded))
        (for _array_element_2 _keys_2
          (Utilities|Map|Add _recapmaterial _array_element_2 (- (.Value (Utilities|Map|Find _recapmaterial _array_element_2)) (.Value (Utilities|Map|Find _matiarlsadded _array_element_2))))
          (Default|SetRecap (Variables|Default|GetGameMode))
          (return (LocalVariables|GetNewLocalVar)))))))