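; BP_ParentStar is the base Blueprint for stars in the craft game mode, showing a shared tooltip widget on cursor hover.
; It caches GM_Craft on BeginPlay, then shows that game mode's star tooltip at the mouse's viewport position and hides it when the cursor leaves.
; StarEffect, SetSelected and SetOverText are empty functions, apparently hooks for child stars.
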(event EventBeginPlay
  (bind _asgm_craft (Utilities|Casting|CastToGM_Craft (Game|GetGameMode)))
  (Utilities|IsValid _asgm_craft
    (:Is%20Valid
      (Variables|Default|SetGameMode _asgm_craft))))

(event Collision|EventActorBeginOverlap
  (params (OtherActor :type Actor%20Object%20Reference)))

(event MouseInput|EventActorBeginCursorOver
  (bind _gamemode (Variables|Default|GetGameMode))
  (bind _widgettooltipstar (Variables|/Game/MyContet/Blueprints/GM_Craft.GM_Craft_C|GetWidgetTooltipStar _gamemode))
  (Widget|SetVisibility _widgettooltipstar "Visible")
  (bind _returnvalue (Class|WidgetLayoutLibrary|GetMousePositiononViewport))
  (Class|CanvasPanelSlot|SetPosition (Class|WidgetLayoutLibrary|SlotasCanvasSlot _widgettooltipstar) _returnvalue))

(event MouseInput|EventActorEndCursorOver
  (Widget|SetVisibility (Variables|/Game/MyContet/Blueprints/GM_Craft.GM_Craft_C|GetWidgetTooltipStar (Variables|Default|GetGameMode)) "Hidden"))

(fn ConstructionScript)

(fn StarEffect)

(fn SetSelected
  (params (IsSelected :type Boolean)))

(fn SetOverText)