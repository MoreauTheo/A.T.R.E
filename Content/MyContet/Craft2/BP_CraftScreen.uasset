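; Crafting screen actor that composites rotatable images through an XOR material and selects the stars lying on bright areas of the result.
; ChangeImage feeds a texture into the rotation material, whose render target becomes the XOR "Add" input on BigPlane.
; ConfirmPose captures the scene and switches the base to the memory render target, while ResetScreen blanks it first.
; Every Tick maps star positions to render target pixels and samples red to set selection.
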(event Custom|ResetScreen
  (bind _mat (Variables|Default|GetMat))
  (Rendering|Material|SetTextureParameterValue _mat "Base" "/Game/MyContet/Blackk.Blackk")
  (Rendering|Material|SetTextureParameterValue _mat "Add" "/Game/MyContet/Blackk.Blackk")
  (CallFunction|ConfirmPose))

(event EventBeginPlay
  (CallFunction|Init))

(event EventTick
  (params (DeltaSeconds :type Float%20%28single-precision%29))
  (CallFunction|ChangeMachin))

(fn ConstructionScript)

(fn LookatPosition
  (params (PixelX :type Integer) (PixelY :type Integer))
  (bind _returnvalue (Class|KismetRenderingLibrary|ReadRenderTargetPixel (Variables|Default|GetRTReel) PixelX PixelY))
  (return (> (.r _returnvalue) 125)))

(fn ChangeMachin
  (bind _bigplane (Variables|Default|GetBigPlane))
  (bind (_min _max) (Components|StaticMesh|GetLocalBounds _bigplane))
  (for _array_element (Variables|/Game/MyContet/Blueprints/GM_Craft.GM_Craft_C|GetCurrentStars (Variables|Default|GetGameMode))
    (bind _isselected (CallFunction|LookatPosition (Math|Float|Truncate (* (/ (- (.x (Variables|/Script/Engine.SceneComponent|GetRelativeLocation (Class|Actor|GetParentComponent _array_element))) (.x _min)) (- (.x _max) (.x _min))) 1748.0)) (Math|Float|Truncate (* (/ (- (.y (Variables|/Script/Engine.SceneComponent|GetRelativeLocation (Class|Actor|GetParentComponent _array_element))) (.y _min)) (- (.y _max) (.y _min))) 1748.0))))
    (Default|SetSelected _array_element _isselected)))

(fn ChangeImage
  (params (NewParam :type Texture%202D%20Object%20Reference))
  (Rendering|Material|SetTextureParameterValue (Variables|Default|GetMaterial%20Rotaion) "TextureToRotate" NewParam)
  (Rendering|Material|SetTextureParameterValue (Variables|Default|GetMat) "Add" "/Game/MyContet/Craft2/RT_Rotation.RT_Rotation"))

(fn Init
  (bind _self self)
  (bind _returnvalue (Transformation|GetActorScale3D _self))
  (bind _asgm_craft (Utilities|Casting|CastToGM_Craft (Game|GetGameMode)))
  (bind _output_get (Variables|Default|SetGameMode _asgm_craft))
  (Variables|/Game/MyContet/Blueprints/GM_Craft.GM_Craft_C|SetCraftScreen _output_get self)
  ;[0 1 0.09461] Material Initialization
  (bind _returnvalue_2 (Rendering|Material|CreateDynamicMaterialInstance "/Game/MyContet/Craft2/M_Xor.M_Xor" "None" "None" :!class /Script/Engine.KismetMaterialLibrary))
  (bind _output_get_2 (Variables|Default|SetMat _returnvalue_2))
  (Rendering|Material|SetTextureParameterValue _output_get_2 "Base" "/Bridge/MSPresets/M_MS_Glass_Material/Textures/Black.Black")
  (Rendering|Material|SetTextureParameterValue (Variables|Default|GetMat) "Add" "/Game/MyContet/Craft2/RT_Rotation.RT_Rotation")
  (Rendering|Material|SetMaterial (Variables|Default|GetBigPlane) 0 (Variables|Default|GetMat))
  (bind _returnvalue_3 (Rendering|Material|CreateDynamicMaterialInstance "/Game/MyContet/Craft2/M_Rotation.M_Rotation" "None" "None" :!class /Script/Engine.KismetMaterialLibrary))
  (bind _output_get_3 (Variables|Default|SetMaterial%20Rotaion _returnvalue_3))
  (Rendering|Material|SetMaterial (Variables|Default|GetPlane2) 0 _output_get_3)
  ;[1 0.4712 0] Capture Camera
  ;;[1 0.2201 0] Capture camera size
  (Variables|/Script/Engine.SceneCaptureComponent2D|SetOrthoWidth (Variables|Default|GetSceneCaptureComponent2D) (* (Variables|/Script/Engine.SceneCaptureComponent2D|GetOrthoWidth (Variables|Default|GetSceneCaptureComponent2D)) (.x _returnvalue)))
  (Variables|/Script/Engine.SceneCaptureComponent2D|SetOrthoWidth (Variables|Default|GetSceneCaptureComponent2D1) (* (Variables|/Script/Engine.SceneCaptureComponent2D|GetOrthoWidth (Variables|Default|GetSceneCaptureComponent2D1)) (.x _returnvalue)))
  ;;[1 0.1721 0.1124] Initialize Capture Camera
  (Rendering|SceneCapture|ShowOnlyComponent (Variables|Default|GetSceneCaptureComponent2D) (Variables|Default|GetBigPlane))
  (Rendering|SceneCapture|CaptureScene (Variables|Default|GetSceneCaptureComponent2D) :!class /Script/Engine.SceneCaptureComponent2D))

(fn ConfirmPose
  (Rendering|SceneCapture|CaptureScene (Variables|Default|GetSceneCaptureComponent2D) :!class /Script/Engine.SceneCaptureComponent2D)
  (Rendering|SceneCapture|CaptureScene (Variables|Default|GetSceneCaptureComponent2D1) :!class /Script/Engine.SceneCaptureComponent2D)
  (Rendering|Material|SetTextureParameterValue (Variables|Default|GetMat) "Add" "/Game/MyContet/Blackk.Blackk")
  (Rendering|Material|SetTextureParameterValue (Variables|Default|GetMat) "Base" "/Game/MyContet/Craft2/RT_Memory.RT_Memory")
  (CallFunction|ChangeMachin))