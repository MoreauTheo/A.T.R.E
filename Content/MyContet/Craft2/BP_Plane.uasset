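; BP_Plane is a prototype actor that combines shape masks on a plane and tests whether a sphere lies in the marked area.
; Keys feed RTMemory and a triangle, round, square or black texture into a dynamic M_Xor material, and T runs two scene captures and clears the added shape.
; T then maps the sphere's position to an RTMemory pixel and swaps its selected or unselected material by the red value.
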(event EventBeginPlay
  (bind _self self)
  (bind _returnvalue (Transformation|GetActorScale3D _self))
  (bind _returnvalue_2 (Rendering|Material|CreateDynamicMaterialInstance "/Game/MyContet/Craft2/M_Xor.M_Xor" "None" "None" :!class /Script/Engine.KismetMaterialLibrary))
  (bind _output_get (Variables|Default|SetMat _returnvalue_2))
  (Rendering|Material|SetTextureParameterValue _output_get "Base" "/Bridge/MSPresets/M_MS_Glass_Material/Textures/Black.Black")
  (Rendering|Material|SetTextureParameterValue (Variables|Default|GetMat) "Add" "/Bridge/MSPresets/M_MS_Glass_Material/Textures/Black.Black")
  (Rendering|Material|SetMaterial (Variables|Default|GetPlane) 0 (Variables|Default|GetMat))
  (Variables|/Script/Engine.SceneCaptureComponent2D|SetOrthoWidth (Variables|Default|GetSceneCaptureComponent2D) (* (Variables|/Script/Engine.SceneCaptureComponent2D|GetOrthoWidth (Variables|Default|GetSceneCaptureComponent2D)) (.x _returnvalue)))
  (Variables|/Script/Engine.SceneCaptureComponent2D|SetOrthoWidth (Variables|Default|GetSceneCaptureComponent2D1) (* (Variables|/Script/Engine.SceneCaptureComponent2D|GetOrthoWidth (Variables|Default|GetSceneCaptureComponent2D1)) (.x _returnvalue)))
  (Rendering|SceneCapture|ShowOnlyComponent (Variables|Default|GetSceneCaptureComponent2D) (Variables|Default|GetPlane))
  (Rendering|SceneCapture|CaptureScene (Variables|Default|GetSceneCaptureComponent2D) :!class /Script/Engine.SceneCaptureComponent2D))

(event Collision|EventActorBeginOverlap
  (params (OtherActor :type Actor%20Object%20Reference)))

(event Input|KeyboardEvents|R
  (params (Key :type Key%20Structure :default "None"))
  (bind _mat (Variables|Default|GetMat))
  (:Pressed
    (Rendering|Material|SetTextureParameterValue _mat "Base" (Variables|Default|GetRTMemory))
    (Rendering|Material|SetTextureParameterValue _mat "Add" "/Game/MyContet/Craft2/ROND.ROND")))

(event Input|KeyboardEvents|V
  (params (Key :type Key%20Structure :default "None"))
  (bind _mat (Variables|Default|GetMat))
  (:Pressed
    (Rendering|Material|SetTextureParameterValue _mat "Base" (Variables|Default|GetRTMemory))
    (Rendering|Material|SetTextureParameterValue _mat "Add" "/Game/MyContet/Craft2/CARRE.CARRE")))

(event Input|KeyboardEvents|P
  (params (Key :type Key%20Structure :default "None"))
  (bind _mat (Variables|Default|GetMat))
  (:Pressed
    (Rendering|Material|SetTextureParameterValue _mat "Base" (Variables|Default|GetRTMemory))
    (Rendering|Material|SetTextureParameterValue _mat "Add" "/Bridge/MSPresets/M_MS_Glass_Material/Textures/Black.Black")))

(event Input|KeyboardEvents|L
  (params (Key :type Key%20Structure :default "None"))
  (:Pressed
    (bind _returnvalue (Class|KismetRenderingLibrary|ReadRenderTargetPixel (Variables|Default|GetRTMemory)))
    (if (> (.b _returnvalue) 125)
      (Development|PrintString "Blanc")
      (else
        (Development|PrintString "Noir")))))

(event Input|KeyboardEvents|T
  (params (Key :type Key%20Structure :default "None"))
  (:Pressed
    (Rendering|SceneCapture|CaptureScene (Variables|Default|GetSceneCaptureComponent2D) :!class /Script/Engine.SceneCaptureComponent2D)
    (Rendering|SceneCapture|CaptureScene (Variables|Default|GetSceneCaptureComponent2D1) :!class /Script/Engine.SceneCaptureComponent2D)
    (Rendering|Material|SetTextureParameterValue (Variables|Default|GetMat) "Add" "/Bridge/MSPresets/M_MS_Glass_Material/Textures/Black.Black")
    (CallFunction|ChangeMachin)))

(event Input|KeyboardEvents|F
  (params (Key :type Key%20Structure :default "None"))
  (bind _mat (Variables|Default|GetMat))
  (:Pressed
    (Rendering|Material|SetTextureParameterValue _mat "Base" (Variables|Default|GetRTMemory))
    (Rendering|Material|SetTextureParameterValue _mat "Add" "/Game/MyContet/Craft2/TRIANGLE.TRIANGLE")))

(fn ConstructionScript)

(fn LookatPosition
  (params (PixelX :type Integer) (PixelY :type Integer))
  (bind _returnvalue (Class|KismetRenderingLibrary|ReadRenderTargetPixel (Variables|Default|GetRTMemory) PixelX PixelY))
  (Development|PrintString (Utilities|String|ToString(Boolean) (> (.r _returnvalue) 125)))
  (return (> (.r _returnvalue) 125)))

(fn ChangeMachin
  (bind _sphere (Variables|Default|GetSphere))
  (bind _plane (Variables|Default|GetPlane))
  (bind (_min _max) (Components|StaticMesh|GetLocalBounds _plane))
  (bind _relativelocation (Variables|/Script/Engine.SceneComponent|GetRelativeLocation _sphere))
  (bind _isselected (CallFunction|LookatPosition (Math|Float|Truncate (* (/ (- (.x _relativelocation) (.x _min)) (- (.x _max) (.x _min))) 1024.0)) (Math|Float|Truncate (* (/ (- (.y _relativelocation) (.y _min)) (- (.y _max) (.y _min))) 1024.0))))
  (if _isselected
    (Rendering|Material|SetMaterial (Variables|Default|GetSphere) 0 (Variables|Default|GetSelectedMaterial))
    (else
      (Rendering|Material|SetMaterial (Variables|Default|GetSphere) 0 (Variables|Default|GetNot%20Selected%20Material)))))