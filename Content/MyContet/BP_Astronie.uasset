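; BP_Astronie is a craftable celestial body that sets up its own crafting data for the GM_Craft game mode.
; On BeginPlay, after the parent's logic, Init registers the actor as the game mode's SelectedBody and names BP_AstroniaCrafted as its product.
; It also fills in orbit rotation speed, size, weight and six Bot/Top value ranges, with no logic here that reads them.
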(event EventBeginPlay
  (|CallParentFunction)
  (CallFunction|Init))

(event Collision|EventActorBeginOverlap
  (params (OtherActor :type Actor%20Object%20Reference))
  (|CallParentFunction OtherActor) ; This node is disabled and will not be called.\nDrag off pins to build functionality.
)

(event EventTick
  (params (DeltaSeconds :type Float%20%28single-precision%29))
  (|CallParentFunction DeltaSeconds) ; This node is disabled and will not be called.\nDrag off pins to build functionality.
)

(fn ConstructionScript
  (|CallParentFunction))

(fn Init
  (bind _asgm_craft (Utilities|Casting|CastToGM_Craft (Game|GetGameMode)))
  (Utilities|IsValid _asgm_craft
    (:Is%20Valid
      (bind _output_get (Variables|Default|SetGameMode _asgm_craft))
      (Variables|/Game/MyContet/GM_Craft.GM_Craft_C|SetSelectedBody _output_get self)
      (Variables|Default|SetProductBody "/Game/MyContet/Blueprints/BP_AstroniaCrafted.BP_AstroniaCrafted_C")
      (Variables|Default|SetRotationSpeedOrbit 2.0)
      (Variables|Default|SetSize 2.0)
      (Variables|Default|SetWeight 2.0)
      (Variables|Default|SetBot1 0.2)
      (Variables|Default|SetTop1 0.3)
      (Variables|Default|SetBot2 0.6)
      (Variables|Default|SetTop2 0.8)
      (Variables|Default|SetBot3 0.25)
      (Variables|Default|SetTop3 0.35)
      (Variables|Default|SetBot4 0.5)
      (Variables|Default|SetTop4 0.9)
      (Variables|Default|SetBot5 0.1)
      (Variables|Default|SetTop5 0.3)
      (Variables|Default|SetBot6 0.7)
      (Variables|Default|SetTop6 1.0))
    (:Is%20Not%20Valid
      (Development|PrintString "GameMode non valide (BP_Astronie)"))))