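; BP_Crank is a mouse-turned crank that drives two progress bars in a crafting UI.
; On BeginPlay it creates the Craft_UI widget, shows the cursor and possesses the Cam actor.
; While held after a click, Tick traces under the cursor and pitches the crank toward the hit, using axis-rotated vectors to read the angle as yaw.
; The frame-to-frame angle change shifts the bars oppositely, ignoring jumps over 180 degrees.
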(event EventBeginPlay
  (bind _returnvalue (Game|ConstructObjectfromClass "/Game/MyContet/Craft_UI.Craft_UI_C"))
  (bind _output_get (Variables|Default|SetUICRaft _returnvalue))
  (UserInterface|Viewport|AddtoViewport _output_get 0)
  (Variables|/Script/Engine.PlayerController|SetbShowMouseCursor (Game|GetPlayerController 0) true)
  (bind _returnvalue_2 (Actor|GetActorOfClass "/Game/MyContet/Cam.Cam_C"))
  (Pawn|Possess (Game|GetPlayerController 0) _returnvalue_2))

(event EventTick
  (params (DeltaSeconds :type Float%20%28single-precision%29))
  (bind _returnvalue (Game|GetPlayerController 0))
  (bind (_worldlocation _worlddirection) (Game|Player|ConvertMouseLocationToWorldSpace _returnvalue))
  (if (Variables|Default|GetTurning)
    (bind _outhit (Collision|LineTraceByChannel _worldlocation (+ _worldlocation (* _worlddirection 1e+04)) "TraceTypeQuery1" true 0 "ForDuration" true "(R=1.000000,G=0.000000,B=0.000000,A=0.000000)"))
    (Transformation|SetActorRotation (Math|Rotator|MakeRotator 0.0 (.Yaw (Math|Rotator|BreakRotator (Math|Rotator|FindLookatRotation (Math|Vector|RotateVectorAroundAxis (Transformation|GetActorLocation) -9e+01 "0.000000,1.000000,0.000000") (Math|Vector|RotateVectorAroundAxis (.impactpoint _outhit) -9e+01 "0.000000,1.000000,0.000000")))) 9e+01) true)
    (Variables|Default|SetRotationTick (- (.Yaw (Math|Rotator|BreakRotator (Math|Rotator|FindLookatRotation (Math|Vector|RotateVectorAroundAxis (Transformation|GetActorLocation) -9e+01 "0.000000,1.000000,0.000000") (Math|Vector|RotateVectorAroundAxis (.impactpoint _outhit) -9e+01 "0.000000,1.000000,0.000000")))) (Variables|Default|GetOldRotation)))
    (if (> (Math|Float|Absolute(Float) (Variables|Default|GetRotationTick)) 1.8e+02)
      _
      (elif (> (Variables|Default|GetRotationTick) 0.0)
        (CallFunction|ChangeBarres (/ (* (Variables|Default|GetRotationTick) DeltaSeconds) 5e+01) (- 0.0 (/ (* (Variables|Default|GetRotationTick) DeltaSeconds) 5e+01)))
        (elif (< (Variables|Default|GetRotationTick) 0.0)
          (CallFunction|ChangeBarres (/ (* (Variables|Default|GetRotationTick) DeltaSeconds) 5e+01) (- 0.0 (/ (* (Variables|Default|GetRotationTick) DeltaSeconds) 5e+01))))))
    (Variables|Default|SetOldRotation (.Yaw (Math|Rotator|BreakRotator (Math|Rotator|FindLookatRotation (Math|Vector|RotateVectorAroundAxis (Transformation|GetActorLocation) -9e+01 "0.000000,1.000000,0.000000") (Math|Vector|RotateVectorAroundAxis (.impactpoint _outhit) -9e+01 "0.000000,1.000000,0.000000")))))))

(event MouseInput|EventActorOnClicked
  (params (ButtonPressed :type Key%20Structure))
  (Development|PrintString "Clicked")
  (Variables|Default|SetTurning true)
  (Variables|Default|SetOldRotation (.pitch (Transformation|GetActorRotation))))

(event Input|MouseEvents|LeftMouseButton
  (params (Key :type Key%20Structure))
  (:Released
    (Variables|Default|SetTurning false)))

(fn ConstructionScript)

(fn ChangeBarres
  (params (Barre1%20Add :type Float%20%28double-precision%29) (Barre2%20Add :type Float%20%28double-precision%29))
  (bind _uicraft (Variables|Default|GetUICRaft))
  (bind _barre1 (Variables|/Game/MyContet/Craft_UI.Craft_UI_C|GetBarre1 _uicraft))
  (bind _barre2 (Variables|/Game/MyContet/Craft_UI.Craft_UI_C|GetBarre2 _uicraft))
  (Progress|SetPercent _barre1 (+ Barre1%20Add (Variables|/Script/UMG.ProgressBar|GetPercent _barre1)))
  (Progress|SetPercent _barre2 (+ Barre2%20Add (Variables|/Script/UMG.ProgressBar|GetPercent _barre2)))
  (return))