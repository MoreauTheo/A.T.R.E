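; Sound manager actor that plays the hub ambience, codex and crafting sound effects, hologram audio and final music through named events.
; On BeginPlay it caches the codex and craft table, whose locations position one-shot and hologram sounds, then fades in the ambience.
; Audio-finished callbacks chain the hologram startup into its follow-up sound and quit the game once the shutdown sound ends.
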(event OnAudioFinished(SFX_StartingHolo_Cue)
  ;[1 1 1] Hologram
  (Audio|Components|Audio|Play (Variables|Default|GetSFX_Holo_Cue) 0.0))

(event OnAudioFinished(SFX_CamTransi_4_Shut_Down_Cue)
  ;[0.2576 1 0.3813] Musique final
  ;;[1 1 1] Quit
  (Game|QuitGame 0 "Quit" false))

(event Custom|Materials_Locked
  ;[1 1 1] Recipe locked / not enough mats
  (Audio|Components|Audio|Play (Variables|Default|GetSfx_Mats_Locked_Cue) 0.0))

(event Custom|Change_Scene
  ;[1 1 1] Movement camera
  (Audio|Components|Audio|Play (Variables|Default|GetSFX_CamTransi_3_Cue) 0.0))

(event Custom|Sound_To_Quit
  ;[0.2576 1 0.3813] Musique final
  ;;[1 1 1] Sound_To_Quit
  (Audio|Components|Audio|Play (Variables|Default|GetSFX_CamTransi_4_Shut_Down_Cue) 0.0))

(event Custom|Crafted_Body
  ;[1 1 1] Crafted Body
  (Audio|PlaySoundatLocation "/Game/MyContet/Sound/Mecanics/SFX_Validate_Body_Cue.SFX_Validate_Body_Cue" (Transformation|GetWorldLocation (Variables|/Game/MyContet/Machines/BP_Table_Craft.BP_Table_Craft_C|GetBP_Button_Craft (Variables|Default|GetTable_Craft_Ref))) "0, 0, 0" 1.0 1.0 0.0 0 0 0 0))

(event Custom|Open_Codex
  ;[1 1 1] Open Codex
  (Audio|PlaySoundatLocation "/Game/MyContet/Sound/Interface/Sfx_UI_Inventory_Open_Cue.Sfx_UI_Inventory_Open_Cue" (Variables|Default|GetLocation_Codex) "0, 0, 0" 1.0 1.0 0.0 0 0 0 0))

(event Custom|Close_Codex
  ;[1 1 1] Close Codex
  (Audio|PlaySoundatLocation "/Game/MyContet/Sound/Interface/Sfx_UI_Inventory_Close_Cue.Sfx_UI_Inventory_Close_Cue" (Variables|Default|GetLocation_Codex) "0, 0, 0" 1.0 1.0 0.0 0 0 0 0)
  (Audio|Components|Audio|AdjustVolume (Variables|Default|GetAmb_Hub_Cue) 3.0 0.35 "Linear" :!class /Script/Engine.AudioComponent))

(event Custom|Final_Music
  ;[0.2576 1 0.3813] Musique final
  (Audio|Components|Audio|FadeOut (Variables|Default|GetAmb_Hub_Cue) 3.0 0.0 "Logarithmic" :!class /Script/Engine.AudioComponent)
  (Audio|Components|Audio|FadeIn (Variables|Default|GetMusic_Final_Cue) 5.0 1.0 0.0 "Linear" :!class /Script/Engine.AudioComponent))

(event Custom|Main_Amb
  ;[0.5233 1 0.5974] Chill main music (il faudra mettre la duration à 15sec pour le jeu final)
  (Audio|Components|Audio|FadeIn (Variables|Default|GetAmb_Hub_Cue) (Variables|Default|GetDuration_Fade_Hub) 1.0 0.0 "Linear" :!class /Script/Engine.AudioComponent))

(event Custom|Choose_Recipe
  ;[1 1 1] Recipe Selected
  (Audio|PlaySoundatLocation "/Game/MyContet/Sound/Interface/SFX_SelectRecipe_Cue.SFX_SelectRecipe_Cue" (Variables|Default|GetLocation_Codex) "0, 0, 0" 1.0 1.0 0.0 0 0 0 0))

(event Custom|Holo_Sound
  ;[1 1 1] Hologram
  (Transformation|SetWorldLocation (Variables|Default|GetSFX_Holo_Cue) (Transformation|GetWorldLocation (Variables|/Game/MyContet/Machines/BP_Table_Craft.BP_Table_Craft_C|GetBP_Button_Craft (Variables|Default|GetTable_Craft_Ref))) false true)
  (Audio|Components|Audio|Play (Variables|Default|GetSFX_StartingHolo_Cue) 0.0))

(event Custom|Ending_Holo
  ;[1 1 1] Hologram
  (Audio|Components|Audio|FadeOut (Variables|Default|GetSFX_Holo_Cue) 0.5 0.0 "Linear" :!class /Script/Engine.AudioComponent))

(event EventBeginPlay
  ;[1 1 1] Event Begin PLay
  (CallFunction|InitSound)
  (CallFunction|MainAmb))

(fn ConstructionScript)

(fn InitSound
  (bind _returnvalue (Actor|GetActorOfClass "/Game/MyContet/Codex/BP_Codex.BP_Codex_C"))
  (Variables|Default|SetCodex_Ref _returnvalue)
  (bind _returnvalue_2 (Actor|GetActorOfClass "/Game/MyContet/Machines/BP_Table_Craft.BP_Table_Craft_C"))
  (Variables|Default|SetTable_Craft_Ref _returnvalue_2)
  (Variables|Default|SetLocation_Codex (Transformation|GetWorldLocation (Variables|/Script/Engine.Actor|GetRootComponent (Variables|Default|GetCodex_Ref)))))