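; Codex icon actor for a celestial or other "Body" entry that spins its mesh and, once unlocked, selects that body through GM_Craft when clicked.
; BeginPlay caches the game mode, creates a hidden WB_CodexOver tooltip, disables actor collision and stops the background flipbook.
; Hovering shows the tooltip and enlarges the background mesh.
; UnlockBody plays the flipbook and Niagara effect, reveals the name and scales the icon in via timeline.
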(event Custom|UnlockBody
  ;[1 0 0] Unlock Body
  (CallFunction|UnlockSelf)
  (bind _scaleicon (Timeline|ScaleIcon Play)
    (:Update
      (Transformation|SetWorldScale3D (Variables|Default|GetSM_BodyIcon) _scaleicon)
      (Variables|Default|SetUnlocked true))))

(event EventBeginPlay
  (bind _asgm_craft (Utilities|Casting|CastToGM_Craft (Game|GetGameMode)))
  (Utilities|IsValid _asgm_craft
    (:Is%20Valid
      (Variables|Default|SetGame%20Mode _asgm_craft)
      (bind _returnvalue (Game|ConstructObjectfromClass "/Game/MyContet/Codex/WB_CodexOver.WB_CodexOver_C"))
      (bind _output_get (Variables|Default|SetTooltip _returnvalue))
      (UserInterface|SetWidget (Variables|Default|GetWB_CodexOver) _output_get)
      (Rendering|SetVisibility (Variables|Default|GetWB_CodexOver) false false)
      (Collision|SetActorEnableCollision false)
      ;[1 1 1] Stop Flipbook Animation
      (CallFunction|StopFlipbook))))

(event EventTick
  (params (DeltaSeconds :type Float%20%28single-precision%29))
  (CallFunction|IconRotation DeltaSeconds))

(event MouseInput|EventActorOnClicked
  (params (ButtonPressed :type Key%20Structure :default "None"))
  (CallFunction|Clicked))

(event Collision|EventActorBeginOverlap
  (params (OtherActor :type Actor%20Object%20Reference)))

(event MouseInput|EventActorBeginCursorOver
  (Rendering|SetVisibility (Variables|Default|GetWB_CodexOver) true false)
  (Default|StartTool (Variables|Default|GetTooltip))
  (Default|SetVariables (Variables|Default|GetTooltip) (Variables|Default|GetBody))
  (Transformation|SetWorldScale3D (Variables|Default|GetSM_BackgroundIcon) "0.180000,0.005000,0.180000")
  (Rendering|SetVisibility (Variables|Default|GetPF_BackgourndIcon) false false))

(event MouseInput|EventActorEndCursorOver
  (Rendering|SetVisibility (Variables|Default|GetWB_CodexOver) false false)
  (Transformation|SetWorldScale3D (Variables|Default|GetSM_BackgroundIcon) "0.150000,0.005000,0.150000")
  (Rendering|SetVisibility (Variables|Default|GetPF_BackgourndIcon) true false))

(fn ConstructionScript)

(fn UnlockSelf
  (bind _pf_backgourndicon (Variables|Default|GetPF_BackgourndIcon))
  (Components|Timeline|PlayfromStart _pf_backgourndicon)
  (Components|Timeline|SetLooping _pf_backgourndicon false)
  (Niagara|SpawnSystematLocation "/Game/MyContet/Codex/Unlock/NS_Unlock.NS_Unlock" (Transformation|GetWorldLocation _pf_backgourndicon) "0.000000,0.000000,60.000000")
  (Development|SetHiddeninGame (Variables|Default|GetTXT_BodyName) false false)
  (Transformation|SetWorldScale3D (Variables|Default|GetSM_BodyIcon) "0, 0, 0"))

(fn StopFlipbook
  (bind _pf_backgourndicon (Variables|Default|GetPF_BackgourndIcon))
  (Utilities|FlowControl|DoOnce false
    (:Completed
      (Components|Timeline|PlayfromStart _pf_backgourndicon)
      (if (== (Class|PaperFlipbookComponent|GetPlaybackPositioninFrames _pf_backgourndicon) 0)
        _
        (else
          _))
      (Audio|Components|Audio|Stop _pf_backgourndicon))))

(fn IconRotation
  (params (DeltaSeconds :type Float%20%28double-precision%29))
  (Transformation|AddLocalRotation (Variables|Default|GetSM_BodyIcon) (Math|Rotator|MakeRotator 0.0 (* (Variables|Default|GetIconRotationSpeed) DeltaSeconds) 0.0) false false))

(fn Clicked
  (if (Variables|Default|GetUnlocked)
    (Default|SelectBody (Variables|Default|GetGame%20Mode) (Variables|Default|GetBody))))