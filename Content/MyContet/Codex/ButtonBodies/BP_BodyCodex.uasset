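; BP_BodyCodex is a clickable actor that represents a Body entry and selects it through the GM_Craft game mode.
; On BeginPlay it caches the game mode and puts a WB_Test1 tooltip into its hidden Widget component.
; Cursor hover shows the tooltip and feeds it the Body, cursor exit hides it, and a click calls SelectBody.
; UnlockSelf is a stub that only prints a message.
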(event EventBeginPlay
  (bind _asgm_craft (Utilities|Casting|CastToGM_Craft (Game|GetGameMode)))
  (Utilities|IsValid _asgm_craft
    (:Is%20Valid
      (Variables|Default|SetGame%20Mode _asgm_craft)
      (bind _returnvalue (Game|ConstructObjectfromClass "/Game/MyContet/Codex/WB_Test1.WB_Test1_C"))
      (bind _output_get (Variables|Default|SetTooltip _returnvalue))
      (UserInterface|SetWidget (Variables|Default|GetWidget) _output_get)
      (Rendering|SetVisibility (Variables|Default|GetWidget) false false))))

(event EventTick
  (params (DeltaSeconds :type Float%20%28single-precision%29)))

(event MouseInput|EventActorOnClicked
  (params (ButtonPressed :type Key%20Structure :default "None"))
  (Default|SelectBody (Variables|Default|GetGame%20Mode) (Variables|Default|GetBody)))

(event Collision|EventActorBeginOverlap
  (params (OtherActor :type Actor%20Object%20Reference)))

(event MouseInput|EventActorBeginCursorOver
  (Rendering|SetVisibility (Variables|Default|GetWidget) true false)
  (Default|StartTool (Variables|Default|GetTooltip))
  (Default|SetVariables (Variables|Default|GetTooltip) (Variables|Default|GetBody)))

(event MouseInput|EventActorEndCursorOver
  (Rendering|SetVisibility (Variables|Default|GetWidget) false false))

(fn ConstructionScript)

(fn UnlockSelf
  (Development|PrintString "Unlocked"))