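; Clickable Pyraxis icon in the Codex whose clicks advance the game's tutorial.
; Its Clicked override calls the parent, then fires Click, which runs two DoOnce gates in sequence.
; The first gate passes one click to allow a tutorial Codex close, set the tutorial material's WeightMask and advance the UI.
; The second starts closed until AllowTutoIcon resets it, then does likewise for the second close step, also updating the description.
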(event Custom|Click
  (bind _game_mode (Variables|Default|GetGame%20Mode))
  (bind _game_mode_2 (Variables|Default|GetGame%20Mode))
  (bind _codex (Variables|/Game/MyContet/Blueprints/GM_Craft.GM_Craft_C|GetCodex _game_mode))
  (bind _ui (Variables|/Game/MyContet/Blueprints/GM_Craft.GM_Craft_C|GetUI _game_mode_2))
  (bind _codex_2 (Variables|/Game/MyContet/Blueprints/GM_Craft.GM_Craft_C|GetCodex _game_mode_2))
  (Utilities|FlowControl|Sequence
    (:then_0
      (Utilities|FlowControl|DoOnce false
        (:Completed
          (Default|AllowTutoCloseCodex _codex)
          (Rendering|Material|SetScalarParameterValue (Variables|/Game/MyContet/Codex/BP_Codex.BP_Codex_C|GetMatTuto _codex) "WeightMask" 1.0 :!class /Script/Engine.MaterialInstanceDynamic)
          (Default|NextTuto (Variables|/Game/MyContet/Blueprints/GM_Craft.GM_Craft_C|GetUI (Variables|Default|GetGame%20Mode))))))
    (:then_1
      (Utilities|FlowControl|DoOnce true
        (:Completed
          (Rendering|Material|SetScalarParameterValue (Variables|/Game/MyContet/Codex/BP_Codex.BP_Codex_C|GetMatTuto _codex_2) "WeightMask" 1.0 :!class /Script/Engine.MaterialInstanceDynamic)
          (Default|NextTuto _ui)
          (Default|SetnextDescription _ui)
          (Default|AllowTutoCloseCodex2 _codex_2))))))

(event Custom|AllowTutoIcon
  (bind _game_mode (Variables|Default|GetGame%20Mode))
  (bind _ui (Variables|/Game/MyContet/Blueprints/GM_Craft.GM_Craft_C|GetUI _game_mode))
  (bind _codex (Variables|/Game/MyContet/Blueprints/GM_Craft.GM_Craft_C|GetCodex _game_mode))
  (Utilities|FlowControl|DoOnce true) ; enters at Reset
)

(event EventBeginPlay
  (|CallParentFunction) ; This node is disabled and will not be called.\nDrag off pins to build functionality.
)

(event Collision|EventActorBeginOverlap
  (params (OtherActor :type Actor%20Object%20Reference))
  (|CallParentFunction OtherActor) ; This node is disabled and will not be called.\nDrag off pins to build functionality.
)

(event EventTick
  (params (DeltaSeconds :type Float%20%28single-precision%29))
  (|CallParentFunction DeltaSeconds) ; This node is disabled and will not be called.\nDrag off pins to build functionality.
)

(fn ConstructionScript
  (|CallParentFunction))

(fn Clicked
  (|CallParentFunction)
  (CallFunction|Click))