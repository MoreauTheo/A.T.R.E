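; BP_Codex is a clickable codex actor that slides open and closed along its local Y axis and registers itself with GM_Craft.
; Clicking its collision calls ToggleCodex, which alternates two timelines that move the root in opposite directions, with CanMove blocking re-triggers until each finishes.
; Movement accumulates as a lerped local offset on every timeline update, scaled by DistanceToMove.
; Each toggle also swaps the four arrow meshes between open and close materials.
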(event OnClicked(Collision)
  (params (TouchedComponent :type Primitive%20Component%20Object%20Reference) (ButtonPressed :type Key%20Structure :default "None"))
  (CallFunction|ToggleCodex))

(event Custom|ToggleCodex
  (if (Variables|Default|GetCan_Move)
    (Variables|Default|SetCan_Move false)
    (CallFunction|ChangeEmissive)
    (Utilities|FlowControl|FlipFlop
      (:A
        (bind _newtrack_0 (Timeline|Timeline_0 PlayFromStart)
          (:Update
            (Transformation|AddLocalOffset (Variables|Default|GetDefaultSceneRoot) (Math|Vector|MakeVector 0.0 (Math|Float|Lerp 0.0 (Variables|Default|GetDistance_To_Move) _newtrack_0) 0.0) false false))
          (:Finished
            (Variables|Default|SetCan_Move true :!label _label))))
      (:B
        (bind _newtrack_0_2 (Timeline|T_Transi PlayFromStart)
          (:Update
            (Transformation|AddLocalOffset (Variables|Default|GetDefaultSceneRoot) (Math|Vector|MakeVector 0.0 (Math|Float|Lerp 0.0 (* -1.0 (Variables|Default|GetDistance_To_Move)) _newtrack_0_2) 0.0) false false))
          (:Finished
            (goto _label)))))))

(event Custom|Change%20emissive
  (bind _arrow_up (Variables|Default|GetArrow_Up))
  (Utilities|FlowControl|FlipFlop
    (:A
      (Rendering|Material|SetMaterial _arrow_up 0 "/Game/MyContet/Leo_Temp/M_Arrow_Open.M_Arrow_Open"))
    (:B
      (Rendering|Material|SetMaterial _arrow_up 0 "/Game/MyContet/Leo_Temp/M_Arrow_Close.M_Arrow_Close"))))

(event EventBeginPlay
  (CallFunction|Init))

(fn ConstructionScript)

(fn Init
  (bind _asgm_craft (Utilities|Casting|CastToGM_Craft (Game|GetGameMode)))
  (Utilities|IsValid _asgm_craft
    (:Is%20Valid
      (bind _output_get (Variables|Default|SetGameMode _asgm_craft))
      (Variables|/Game/MyContet/Blueprints/GM_Craft.GM_Craft_C|SetCodex _output_get self))
    (:Is%20Not%20Valid
      (Development|PrintString "GameMode non valide (BP_Crank)"))))