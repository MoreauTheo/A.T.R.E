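; BP_MaterialWheel is a rotatable wheel actor that holds BP_Material child actors.
; On BeginPlay, Init walks the static mesh's child actor components and gives each BP_Material a reference back to the wheel.
; Cursor events on the Cylinder set a hover flag.
; While hovered, Tick pitches the static mesh by a negated input axis value, scaled by scrolling speed and delta time.
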(event OnBeginCursorOver(Cylinder)
  (params (TouchedComponent :type Primitive%20Component%20Object%20Reference))
  (Variables|Default|SetHovered true))

(event OnEndCursorOver(Cylinder)
  (params (TouchedComponent :type Primitive%20Component%20Object%20Reference))
  (Variables|Default|SetHovered false))

(event EventBeginPlay
  (CallFunction|Init))

(event EventTick
  (params (DeltaSeconds :type Float%20%28single-precision%29))
  (if (Variables|Default|GetHovered)
    (CallFunction|Turn)))

(fn ConstructionScript)

(fn Init
  (for _array_element (Components|GetChildrenComponents (Variables|Default|GetStaticMesh) false)
    (bind _aschild_actor_component (Utilities|Casting|CastToChildActorComponent _array_element))
    (bind _asbp_material (Utilities|Casting|CastToBP_Material (Variables|/Script/Engine.ChildActorComponent|GetChildActor _aschild_actor_component)))
    (Variables|/Game/MyContet/Materiaux/BP_Material.BP_Material_C|SetMaterialWheel _asbp_material self)))

(fn ApplyMaterialWheelVariabletoChild
  (params (Child :type BP%20Material%20Object%20Reference))
  (Variables|/Game/MyContet/Materiaux/BP_Material.BP_Material_C|SetMaterialWheel Child self))

(fn Turn
  (Transformation|AddLocalRotation (Variables|Default|GetStaticMesh) (Math|Rotator|MakeRotator 0.0 (* (Utilities|Time|GetWorldDeltaSeconds) (* (- 0.0 (Class|Actor|GetInputAxisKeyValue)) (Variables|Default|GetScrollingSpeed))) 0.0) false false))