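; BP_EndRound is an end-of-round Blueprint that toggles the visibility of a winnings panel.
; On BeginPlay it enables input from player controller 0, then handles raw key presses directly.
; B calls ShowWinnings and V calls UnshowWinnings, which set the visibility of WinningsPannel and its children.
; The file contains no round-end detection or winnings calculation.
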(event EventBeginPlay
  (Input|EnableInput (Game|GetPlayerController 0)))

(event Input|KeyboardEvents|B
  (params (Key :type Key%20Structure))
  (:Pressed
    (CallFunction|ShowWinnings)))

(event Input|KeyboardEvents|V
  (params (Key :type Key%20Structure))
  (:Pressed
    (CallFunction|UnshowWinnings)))

(fn ConstructionScript)

(fn ShowWinnings
  (Rendering|SetVisibility (Variables|Default|GetWinningsPannel) true true))

(fn UnshowWinnings
  (Rendering|SetVisibility (Variables|Default|GetWinningsPannel) false true))