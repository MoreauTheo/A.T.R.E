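; BP_AstroniaCrafted is a crafted Astronia body that derives a debug color from its three effect slots.
; On Start it calls Init, then SetColor maps Effet1, Effet2 and Effet3 to red, green and blue at zero, half or full intensity.
; SetColor then creates a dynamic instance of M_BodyDebug, stores it in MaterialI and writes the color to its ColorDebug parameter.
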(event EventBeginPlay
  (|CallParentFunction))

(event Collision|EventActorBeginOverlap
  (params (OtherActor :type Actor%20Object%20Reference))
  (|CallParentFunction OtherActor) ; This node is disabled and will not be called.\nDrag off pins to build functionality.
)

(event EventTick
  (params (DeltaSeconds :type Float%20%28single-precision%29))
  (|CallParentFunction DeltaSeconds))

(event EventStart
  (CallFunction|Init)
  (CallFunction|SetColor))

(fn ConstructionScript
  (|CallParentFunction))

(fn SetColor
  (switch Utilities|FlowControl|Switch|SwitchonE_EffectPossibility (Variables|Default|GetEffet1)
    (:NewEnumerator0
      (LocalVariables|SetColor (Math|Vector|MakeVector 0.0 (.y (LocalVariables|GetColor)) (.z (LocalVariables|GetColor)))))
    (:NewEnumerator1
      (LocalVariables|SetColor (Math|Vector|MakeVector 0.5 (.y (LocalVariables|GetColor)) (.z (LocalVariables|GetColor)))))
    (:NewEnumerator2
      (LocalVariables|SetColor (Math|Vector|MakeVector 1.0 (.y (LocalVariables|GetColor)) (.z (LocalVariables|GetColor))))))
  (switch Utilities|FlowControl|Switch|SwitchonE_EffectPossibility (Variables|Default|GetEffet2)
    (:NewEnumerator0
      (LocalVariables|SetColor (Math|Vector|MakeVector (.x (LocalVariables|GetColor)) 0.0 (.z (LocalVariables|GetColor)))))
    (:NewEnumerator1
      (LocalVariables|SetColor (Math|Vector|MakeVector (.x (LocalVariables|GetColor)) 0.5 (.z (LocalVariables|GetColor)))))
    (:NewEnumerator2
      (LocalVariables|SetColor (Math|Vector|MakeVector (.x (LocalVariables|GetColor)) 1.0 (.z (LocalVariables|GetColor))))))
  (switch Utilities|FlowControl|Switch|SwitchonE_EffectPossibility (Variables|Default|GetEffet3)
    (:NewEnumerator0
      (LocalVariables|SetColor (Math|Vector|MakeVector (.x (LocalVariables|GetColor)) (.y (LocalVariables|GetColor)) 0.0)))
    (:NewEnumerator1
      (LocalVariables|SetColor (Math|Vector|MakeVector (.x (LocalVariables|GetColor)) (.y (LocalVariables|GetColor)) 0.5)))
    (:NewEnumerator2
      (LocalVariables|SetColor (Math|Vector|MakeVector (.x (LocalVariables|GetColor)) (.y (LocalVariables|GetColor)) 1.0))))
  (bind _returnvalue (Rendering|Material|CreateDynamicMaterialInstance "/Game/MyContet/GraphicMaterial/M_BodyDebug.M_BodyDebug" "None" "None" :!class /Script/Engine.KismetMaterialLibrary))
  (bind _output_get (LocalVariables|SetMaterialI _returnvalue))
  (Rendering|Material|SetVectorParameterValue _returnvalue "ColorDebug" (Utilities|Struct|MakeLinearColor (.x (LocalVariables|GetColor)) (.y (LocalVariables|GetColor)) (.z (LocalVariables|GetColor)) 1.0) :!class /Script/Engine.MaterialInstanceDynamic))