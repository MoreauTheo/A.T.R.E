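; BP_Prismor_Crafted is the Prismor planet actor, with two rotating asteroid belts and a destruction effect triggered by the C key.
; Tick spins each belt around its local pitch axis at its own speed, scaled by delta time.
; Pressing C swaps the skeletal mesh for the GCPrismor geometry collection, crumbles its active clusters and spawns an explosion system at a fixed offset from it.
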(event EventBeginPlay
  (|CallParentFunction))

(event Collision|EventActorBeginOverlap
  (params (OtherActor :type Actor%20Object%20Reference))
  (|CallParentFunction OtherActor) ; This node is disabled and will not be called.\nDrag off pins to build functionality.
)

(event EventTick
  (params (DeltaSeconds :type Float%20%28single-precision%29))
  (|CallParentFunction DeltaSeconds)
  ;[1 1 1] Belt Rotation
  (Transformation|AddLocalRotation (Variables|Default|GetSM_AsteroidBelt) (Math|Rotator|MakeRotator 0.0 (* (Variables|AsteroidBelt|GetSpeed) DeltaSeconds) 0.0) false false)
  (Transformation|AddLocalRotation (Variables|Default|GetSM_AsteroidBelt1) (Math|Rotator|MakeRotator 0.0 (* (Variables|AsteroidBelt|GetSpeed_0) DeltaSeconds) 0.0) false false))

(event Input|KeyboardEvents|C
  (params (Key :type Key%20Structure :default "None"))
  (bind _gc_prismor (Variables|Default|GetGC_Prismor))
  (:Pressed
    ;[1 1 1] Planet Explosion
    (Development|SetHiddeninGame _gc_prismor false false)
    (Development|SetHiddeninGame (Variables|Default|GetSkeletalMesh) true false)
    (Class|GeometryCollectionComponent|CrumbleActiveClusters _gc_prismor)
    (Niagara|SpawnSystematLocation "/Game/MyContet/VFX/Explosion/NS_Explosion.NS_Explosion" (+ (Transformation|GetWorldLocation _gc_prismor) "47000.000000,47000.000000,0.000000") "90.000000,0.000000,0.000000")))

(fn ConstructionScript
  (|CallParentFunction))