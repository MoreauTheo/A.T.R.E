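; BP_LifeBar is a world-space gauge actor that displays a quantity, apparently lifetime, as a progress bar.
; On BeginPlay it creates a WBP_LifetimeJauge widget and assigns it to its Widget component.
; The SetQuantity event writes its input directly to the progress bar's percent.
; Every Tick it rotates the whole actor toward the Camera's location, so the bar always faces the view.
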(event Custom|SetQuantity
  (params (QuantityInput :type Float%20%28double-precision%29))
  (Variables|/Script/UMG.ProgressBar|SetPercent (Variables|/Game/MyContet/Bodies/WBP_LifetimeJauge.WBP_LifetimeJauge_C|GetProgressBar_114 (Variables|Default|GetWidgetBar)) QuantityInput))

(event EventBeginPlay
  (bind _returnvalue (Game|ConstructObjectfromClass "/Game/MyContet/Bodies/WBP_LifetimeJauge.WBP_LifetimeJauge_C"))
  (bind _output_get (Variables|Default|SetWidgetBar _returnvalue))
  (UserInterface|SetWidget (Variables|Default|GetWidget) _output_get))

(event Collision|EventActorBeginOverlap
  (params (OtherActor :type Actor%20Object%20Reference)))

(event EventTick
  (params (DeltaSeconds :type Float%20%28single-precision%29))
  (Transformation|SetActorRotation (Math|Rotator|FindLookatRotation (Transformation|GetActorLocation) (Transformation|GetActorLocation (Variables|Default|GetCamera)))))

(fn ConstructionScript)