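; BP_Hexor_Crafted is the crafted Hexor body, a child Blueprint with a spinning asteroid belt.
; Tick runs the parent logic, then rotates the belt mesh in local pitch by Speed and the skeletal mesh in local yaw by SpeedBody, both scaled by delta time.
; BeginPlay and the construction script only call the parent, and the overlap event is disabled.
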(event EventBeginPlay
  (|CallParentFunction))

(event Collision|EventActorBeginOverlap
  (params (OtherActor :type Actor%20Object%20Reference))
  (|CallParentFunction OtherActor) ; This node is disabled and will not be called.\nDrag off pins to build functionality.
)

(event EventTick
  (params (DeltaSeconds :type Float%20%28single-precision%29))
  (|CallParentFunction DeltaSeconds)
  ;[1 1 1] Belt Rotation
  (Transformation|AddLocalRotation (Variables|Default|GetSM_AsteroidBelt) (Math|Rotator|MakeRotator 0.0 (* (Variables|AsteroidBelt|GetSpeed) DeltaSeconds) 0.0) false false)
  (Transformation|AddLocalRotation (Variables|Default|GetSkeletalMesh) (Math|Rotator|MakeRotator 0.0 0.0 (* (Variables|Default|GetSpeed_Body) DeltaSeconds)) false false))

(fn ConstructionScript
  (|CallParentFunction))