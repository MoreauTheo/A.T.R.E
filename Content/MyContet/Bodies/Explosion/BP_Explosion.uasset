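; BP_Explosion is a key-triggered destruction test actor that blows apart a Geometry Collection.
; It enables player input on BeginPlay, and pressing C calls Explosion.
; That function crumbles GCTest's active clusters, applies an enormous constant-falloff radial impulse at its location and spawns the NS_Explosion Niagara effect.
; Parallel timers from a Sequence hide SMAsteroidBelt1 shortly afterward and destroy the GCTest component later.
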(event EventBeginPlay
  ;[1 0.3478 0] Key Test
  (Input|EnableInput (Game|GetPlayerController 0)))

(event Input|KeyboardEvents|C
  (params (Key :type Key%20Structure :default "None"))
  (:Pressed
    ;[1 1 1] Explosion
    (Utilities|FlowControl|Sequence
      (:then_0
        (CallFunction|Explosion)
        (Utilities|FlowControl|Delay 2e+01)
        (Components|DestroyComponent (Variables|Default|GetGC_Test)))
      (:then_1
        (Utilities|FlowControl|Delay 2.0)
        (Development|SetHiddeninGame (Variables|Default|GetSM_AsteroidBelt1) true false)))))

(fn ConstructionScript)

(fn Explosion
  (bind _gc_test (Variables|Default|GetGC_Test))
  (bind _returnvalue (Transformation|GetWorldLocation _gc_test))
  (Class|GeometryCollectionComponent|CrumbleActiveClusters _gc_test)
  (Physics|AddRadialImpulse _gc_test _returnvalue 9e+08 9e+08 "RIF_Constant" false)
  (Niagara|SpawnSystematLocation "/Game/MyContet/Bodies/Explosion/NS_Explosion.NS_Explosion" _returnvalue "90.000000,0.000000,0.000000"))