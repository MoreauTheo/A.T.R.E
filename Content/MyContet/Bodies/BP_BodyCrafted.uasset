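; Base crafted body that can orbit the black hole along its spline and award materials to the player.
; Init caches the GM_Craft game mode, the BlackHole spline and the actor's starting distance along it.
; Orbit steps that distance backwards by speed and delta time, moving the root to the spline location.
; GiveMaterials passes each MaterialGainTab entry to the game mode's UpdateQuantity; neither function is called within this Blueprint.
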(event Custom|Start)

(event EventBeginPlay
  (CallFunction|Init))

(event Collision|EventActorBeginOverlap
  (params (OtherActor :type Actor%20Object%20Reference)))

(event EventTick
  (params (DeltaSeconds :type Float%20%28single-precision%29)))

(fn ConstructionScript)

(fn Init
  (bind _asgm_craft (Utilities|Casting|CastToGM_Craft (Game|GetGameMode)))
  (Utilities|IsValid _asgm_craft
    (:Is%20Valid
      (bind _output_get (Variables|Default|SetGameMode _asgm_craft))
      (bind _output_get_2 (Variables|Default|SetSplineOrbit (Variables|/Game/MyContet/Bodies/BlackHole/BP_BlackHole.BP_BlackHole_C|GetSpline (Variables|/Game/MyContet/Blueprints/GM_Craft.GM_Craft_C|GetBlackHole _output_get))))
      (Variables|Default|SetStartPosition (Class|SplineComponent|GetDistanceAlongSplineatLocation _output_get_2 (Transformation|GetActorLocation) "World"))
      (Variables|Default|SetMeshSkeletal (Variables|/Script/Engine.SkeletalMeshComponent|GetSkeletalMeshAsset (Variables|Default|GetSkeletalMesh))))
    (:Is%20Not%20Valid
      (Development|PrintString "GameMode non valide (BP_Crank)"))))

(fn Orbit
  (Transformation|SetWorldTransform (Variables|Default|GetDefaultSceneRoot) (Math|Transform|MakeTransform (.location (Spline|GetTransformatDistanceAlongSpline (Variables|Default|GetSplineOrbit) (Variables|Default|GetStartPosition) "World" false)) "0, 0, 0" "1.000000,1.000000,1.000000") false false)
  (Variables|Default|SetStartPosition (- (Variables|Default|GetStartPosition) (* (Utilities|Time|GetWorldDeltaSeconds) (Variables|Default|GetSpeedOrbit)))))

(fn GiveMaterials
  (bind _materialgaintab (Variables|Default|GetMaterialGainTab))
  (bind _keys (Utilities|Map|Keys _materialgaintab))
  (for (_array_element _array_index) _keys
    (bind _values (Utilities|Map|Values _materialgaintab))
    (Default|UpdateQuantity (Variables|Default|GetGameMode) _array_element (Utilities|Array|Get(acopy) _values _array_index))))