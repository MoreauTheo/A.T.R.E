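; BP_ZentorCrafted is the Zentor body actor, a skeletal mesh with two asteroid belt components that spin continuously.
; After calling the parent Tick, it adds frame-rate-independent local rotation to each component.
; Each belt turns equally on roll, pitch and yaw at its own speed, while the body turns only on yaw at a separate speed.
; The construction script only calls the parent.
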(event EventTick
  (params (DeltaSeconds :type Float%20%28single-precision%29))
  (bind _speed (Variables|AsteroidBelt|GetSpeed))
  (bind _speed1 (Variables|AsteroidBelt|GetSpeed1))
  (bind _returnvalue (* _speed1 DeltaSeconds))
  (bind _returnvalue_2 (* _speed DeltaSeconds))
  (|CallParentFunction DeltaSeconds)
  ;[1 1 1] Belt Rotation
  (Utilities|FlowControl|Sequence
    (:then_0
      (Transformation|AddLocalRotation (Variables|Default|GetSM_AsteroidBelt) (Math|Rotator|MakeRotator _returnvalue_2 _returnvalue_2 _returnvalue_2) false false))
    (:then_1
      (Transformation|AddLocalRotation (Variables|Default|GetSM_AsteroidBelt1) (Math|Rotator|MakeRotator _returnvalue _returnvalue _returnvalue) false false))
    (:then_2
      ;;[1 1 1] Zentor Rotation
      (Transformation|AddLocalRotation (Variables|Default|GetSkeletalMesh) (Math|Rotator|MakeRotator 0.0 0.0 (* (Variables|Default|GetSpeed_Body) DeltaSeconds)) false false))))

(fn ConstructionScript
  (|CallParentFunction))