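; Blueprint for the crafted Vyranis celestial body, with two rotating asteroid belts and a key-triggered planet explosion.
; Tick spins both belt meshes locally in roll and pitch, scaled by Speed and delta time.
; Pressing C swaps the skeletal mesh for the GCZentor Geometry Collection, crumbles its active clusters and spawns a Niagara explosion at a fixed offset from it.
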(event EventBeginPlay
  (|CallParentFunction))

(event Collision|EventActorBeginOverlap
  (params (OtherActor :type Actor%20Object%20Reference))
  (|CallParentFunction OtherActor) ; This node is disabled and will not be called.\nDrag off pins to build functionality.
)

(event EventTick
  (params (DeltaSeconds :type Float%20%28single-precision%29))
  (bind _speed (Variables|AsteroidBelt|GetSpeed))
  (bind _returnvalue (* _speed DeltaSeconds))
  (bind _returnvalue_2 (Math|Rotator|MakeRotator _returnvalue _returnvalue 0.0))
  (|CallParentFunction DeltaSeconds)
  ;[1 1 1] Belt Rotation
  (Transformation|AddLocalRotation (Variables|Default|GetSM_AsteroidBelt) _returnvalue_2 false false)
  (Transformation|AddLocalRotation (Variables|Default|GetSM_AsteroidBelt1) _returnvalue_2 false false))

(event Input|KeyboardEvents|C
  (params (Key :type Key%20Structure :default "None"))
  (bind _gc_zentor (Variables|Default|GetGC_Zentor))
  (:Pressed
    ;[1 1 1] Planet Explosion
    (Development|SetHiddeninGame _gc_zentor false false)
    (Development|SetHiddeninGame (Variables|Default|GetSkeletalMesh) true false)
    (Class|GeometryCollectionComponent|CrumbleActiveClusters _gc_zentor)
    (Niagara|SpawnSystematLocation "/Game/MyContet/Bodies/Explosion/NS_Explosion.NS_Explosion" (+ (Transformation|GetWorldLocation _gc_zentor) "55000.000000,55000.000000,0.000000") "90.000000,0.000000,0.000000")))

(fn ConstructionScript
  (|CallParentFunction))