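; BP_Metiron_Crafted is the Blueprint for a crafted Metiron body with a spinning asteroid belt.
; Each Tick runs the parent logic, then rotates the SMAsteroidBelt component locally on roll, pitch and yaw by Speed scaled by delta time.
; The construction script only calls its parent, and the BeginPlay and overlap events are disabled stubs.
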(event EventBeginPlay
  (|CallParentFunction) ; This node is disabled and will not be called.\nDrag off pins to build functionality.
)

(event Collision|EventActorBeginOverlap
  (params (OtherActor :type Actor%20Object%20Reference))
  (|CallParentFunction OtherActor) ; This node is disabled and will not be called.\nDrag off pins to build functionality.
)

(event EventTick
  (params (DeltaSeconds :type Float%20%28single-precision%29))
  (bind _speed (Variables|Default|GetSpeed))
  (bind _returnvalue (* _speed DeltaSeconds))
  (|CallParentFunction DeltaSeconds)
  ;[1 1 1] Belt Rotation
  (Transformation|AddLocalRotation (Variables|Default|GetSM_AsteroidBelt) (Math|Rotator|MakeRotator _returnvalue _returnvalue _returnvalue) false false))

(fn ConstructionScript
  (|CallParentFunction))