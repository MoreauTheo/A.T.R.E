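; Actor for the crafted Nexus, which triggers the craft scene's black hole explosion when it begins play.
; On BeginPlay it casts the game mode to GM_Craft, caches it and calls BlackHoleExplosion on that game mode's BlackHole.
; It then turns off collision on the parts of the game mode's down scene arrow, ArrowSceneDown.
; Overlap and Tick events are disabled, so all logic runs once at spawn.
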(event EventBeginPlay
  (|CallParentFunction)
  (bind _asgm_craft (Utilities|Casting|CastToGM_Craft (Game|GetGameMode)))
  (Variables|Default|SetAs%20GM%20Craft _asgm_craft)
  (Default|BlackHoleExplosion (Variables|/Game/MyContet/Blueprints/GM_Craft.GM_Craft_C|GetBlackHole (Variables|Default|GetAs%20GM%20Craft)))
  (Collision|SetCollisionEnabled (Variables|/Game/MyContet/ChangeScenes/BP_ArrowSceneDown.BP_ArrowSceneDown_C|GetCube (Variables|/Game/MyContet/Blueprints/GM_Craft.GM_Craft_C|GetArrowSceneDown (Variables|Default|GetAs%20GM%20Craft))) "NoCollision")
  (Collision|SetCollisionEnabled (Variables|/Game/MyContet/ChangeScenes/BP_ArrowSceneDown.BP_ArrowSceneDown_C|GetFleche (Variables|/Game/MyContet/Blueprints/GM_Craft.GM_Craft_C|GetArrowSceneDown (Variables|Default|GetAs%20GM%20Craft))) "NoCollision")
  (Collision|SetCollisionEnabled (Variables|/Game/MyContet/ChangeScenes/BP_ArrowSceneDown.BP_ArrowSceneDown_C|GetLightBeveled (Variables|/Game/MyContet/Blueprints/GM_Craft.GM_Craft_C|GetArrowSceneDown (Variables|Default|GetAs%20GM%20Craft))) "NoCollision"))

(event Collision|EventActorBeginOverlap
  (params (OtherActor :type Actor%20Object%20Reference))
  (|CallParentFunction OtherActor) ; This node is disabled and will not be called.\nDrag off pins to build functionality.
)

(event EventTick
  (params (DeltaSeconds :type Float%20%28single-precision%29))
  (|CallParentFunction DeltaSeconds) ; This node is disabled and will not be called.\nDrag off pins to build functionality.
)

(fn ConstructionScript
  (|CallParentFunction))