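; BP_Window is an interface window actor whose screens are shown and hidden with keyboard keys.
; On BeginPlay it enables input from player controller 0, then L calls UnhiddeInterface and K calls HiddeInterface.
; Each function sets the Screens component's hidden state, propagated to its children, and changes the EmissiveIntensity material parameter on SMButton so the button glows brightly when shown and dims when hidden.
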(event EventBeginPlay
  (Input|EnableInput (Game|GetPlayerController 0)))

(event Input|KeyboardEvents|L
  (params (Key :type Key%20Structure :default "None"))
  (:Pressed
    ;[1 1 1] Hidde / Unhidde screens
    (CallFunction|UnhiddeInterface)))

(event Input|KeyboardEvents|K
  (params (Key :type Key%20Structure :default "None"))
  (:Pressed
    ;[1 1 1] Hidde / Unhidde screens
    (CallFunction|HiddeInterface)))

(fn ConstructionScript)

(fn HiddeInterface
  (Rendering|Material|SetScalarParameterValueonMaterials (Variables|Default|GetSM_Button) "EmissiveIntensity" 0.1)
  (Development|SetHiddeninGame (Variables|Default|GetScreens) true true))

(fn UnhiddeInterface
  (Rendering|Material|SetScalarParameterValueonMaterials (Variables|Default|GetSM_Button) "EmissiveIntensity" 1.0)
  (Development|SetHiddeninGame (Variables|Default|GetScreens) false true))